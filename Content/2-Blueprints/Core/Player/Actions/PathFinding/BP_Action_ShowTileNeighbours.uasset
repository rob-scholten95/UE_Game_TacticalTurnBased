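; A player action that highlights the valid neighbours of a given grid tile through a tile state, likely as a pathfinding visual aid.
; ExecuteAction clears that state from the grid, asks the grid's pathfinding component for neighbours of allowed tile types, optionally including diagonals, then adds the state to each.
; EndPlay runs the action with an off-grid index, so the highlight is cleared when the action ends.
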(event EventBeginPlay
  (|CallParentFunction) ; This node is disabled and will not be called.\nDrag off pins to build functionality.
)

(event Collision|EventActorBeginOverlap
  (params (OtherActor :type Actor%20Object%20Reference))
  (|CallParentFunction OtherActor) ; This node is disabled and will not be called.\nDrag off pins to build functionality.
)

(event EventTick
  (params (DeltaSeconds :type Float%20%28single-precision%29))
  (|CallParentFunction DeltaSeconds) ; This node is disabled and will not be called.\nDrag off pins to build functionality.
)

(event EventEndPlay
  (params (EndPlayReason :type EEndPlayReason%20Enum :default "Destroyed"))
  (CallFunction|ExecuteAction (Utilities|Struct|MakeIntPoint -999 -999)))

(fn ConstructionScript
  (|CallParentFunction))

(fn ExecuteAction
  (params (Index :type Int%20Point%20Structure))
  (Default|ClearStatefromTiles (Variables|/Game/2-Blueprints/Core/Player/BP_PlayerActions.BP_PlayerActions_C|GetBP_Grid (Variables|Default|GetBP_PlayerActions)) "NewEnumerator3")
  (bind _neighbours (Default|GetValidTileNeighbors (Variables|/Game/2-Blueprints/Core/Grid/BP_Grid.BP_Grid_C|GetBP_GridPathFinding (Variables|/Game/2-Blueprints/Core/Player/BP_PlayerActions.BP_PlayerActions_C|GetBP_Grid (Variables|Default|GetBP_PlayerActions))) Index (Variables|Default|GetInclude%20Diagonals) (Utilities|Array|MakeArray "NewEnumerator1" "NewEnumerator4" "NewEnumerator5" "NewEnumerator6")))
  (for _array_element _neighbours
    (Default|AddStatetoTile (Variables|/Game/2-Blueprints/Core/Player/BP_PlayerActions.BP_PlayerActions_C|GetBP_Grid (Variables|Default|GetBP_PlayerActions)) (.index _array_element) "NewEnumerator3")))