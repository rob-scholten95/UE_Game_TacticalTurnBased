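; Player action that moves the selected unit across the combat grid to a chosen tile.
; It requests a path from the grid's pathfinder using the unit's diagonal, tile-type and current MP stats.
; When the path completes, it marks those tiles, has the combat system move the unit and calls ResetMP.
; Path highlights clear when walking finishes or the action re-executes, including with an off-grid index on EndPlay.
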(event EventBeginPlay
  (|CallParentFunction) ; This node is disabled and will not be called.\nDrag off pins to build functionality.
)

(event Collision|EventActorBeginOverlap
  (params (OtherActor :type Actor%20Object%20Reference))
  (|CallParentFunction OtherActor) ; This node is disabled and will not be called.\nDrag off pins to build functionality.
)

(event EventTick
  (params (DeltaSeconds :type Float%20%28single-precision%29))
  (|CallParentFunction DeltaSeconds) ; This node is disabled and will not be called.\nDrag off pins to build functionality.
)

(event EventEndPlay
  (params (EndPlayReason :type EEndPlayReason%20Enum :default "Destroyed"))
  (CallFunction|ExecuteAction (Utilities|Struct|MakeIntPoint -999 -999)))

(fn ConstructionScript
  (|CallParentFunction))

(fn ExecuteAction
  (params (Index :type Int%20Point%20Structure))
  (bind _bp_playeractions (Variables|Default|GetBP_PlayerActions))
  (bind _selectedunit (Variables|/Game/2-Blueprints/Core/Player/BP_PlayerActions.BP_PlayerActions_C|GetSelectedUnit _bp_playeractions))
  (Default|ClearStatefromTiles (Variables|/Game/2-Blueprints/Core/Player/BP_PlayerActions.BP_PlayerActions_C|GetBP_Grid (Variables|Default|GetBP_PlayerActions)) "NewEnumerator4")
  (Variables|Default|SetCurrent%20Unit _selectedunit)
  (Utilities|IsValid _selectedunit
    (:Is%20Valid
      (EventDispatchers|BindEventtoOnUnitFinishedWalking (Variables|Default|GetCurrent%20Unit) (EventDispatchers|CreateEvent :!event OnUnitFinishedWalking))
      (EventDispatchers|BindEventtoOnPathFindingCompleted (Variables|/Game/2-Blueprints/Core/Grid/BP_Grid.BP_Grid_C|GetBP_GridPathFinding (Variables|/Game/2-Blueprints/Core/Player/BP_PlayerActions.BP_PlayerActions_C|GetBP_Grid (Variables|Default|GetBP_PlayerActions))) (EventDispatchers|CreateEvent :!event OnPathFindingCompleted))
      (Default|FindPath (Variables|/Game/2-Blueprints/Core/Grid/BP_Grid.BP_Grid_C|GetBP_GridPathFinding (Variables|/Game/2-Blueprints/Core/Player/BP_PlayerActions.BP_PlayerActions_C|GetBP_Grid (Variables|Default|GetBP_PlayerActions))) (Variables|/Game/2-Blueprints/Core/Player/BP_PlayerActions.BP_PlayerActions_C|GetSelectedTileIndex (Variables|Default|GetBP_PlayerActions)) Index (.CanMoveDiagonally (Utilities|Struct|BreakSTR_UnitData_Stats (Utilities|Struct|BreakSTR_UnitData (Variables|/Game/2-Blueprints/Core/Units/BP_Unit.BP_Unit_C|GetUnitData (Variables|Default|GetCurrent%20Unit))))) 0.0 0.0 (.ValidTileTypes (Utilities|Struct|BreakSTR_UnitData_Stats (Utilities|Struct|BreakSTR_UnitData (Variables|/Game/2-Blueprints/Core/Units/BP_Unit.BP_Unit_C|GetUnitData (Variables|Default|GetCurrent%20Unit))))) false (.MP_Current (Utilities|Struct|BreakSTR_UnitData_Stats (Utilities|Struct|BreakSTR_UnitData (Variables|/Game/2-Blueprints/Core/Units/BP_Unit.BP_Unit_C|GetUnitData (Variables|Default|GetCurrent%20Unit)))))))))

(fn OnPathFindingCompleted
  (params (Path :type Array%20of%20Int%20Point%20Structures))
  (bind _current_unit (Variables|Default|GetCurrent%20Unit))
  (if (== (Variables|Default|GetCurrent%20Unit) (Variables|/Game/2-Blueprints/Core/Player/BP_PlayerActions.BP_PlayerActions_C|GetSelectedUnit (Variables|Default|GetBP_PlayerActions)))
    (Utilities|IsValid (Variables|Default|GetCurrent%20Unit)
      (:Is%20Valid
        (for _array_element Path
          (Default|AddStatetoTile (Variables|/Game/2-Blueprints/Core/Player/BP_PlayerActions.BP_PlayerActions_C|GetBP_Grid (Variables|Default|GetBP_PlayerActions)) _array_element "NewEnumerator4"))
        (Variables|/Game/2-Blueprints/Core/Units/BP_Unit.BP_Unit_C|SetMoveDurationPerTile (Variables|Default|GetCurrent%20Unit) (Variables|Default|GetMove%20Duration%20Per%20Tile))
        (Default|MoveUnit (Variables|/Game/2-Blueprints/Core/Player/BP_PlayerActions.BP_PlayerActions_C|GetBP_CombatSystem (Variables|Default|GetBP_PlayerActions)) _current_unit Path)
        (Default|ResetMP _current_unit)))))

(fn OnUnitFinishedWalking
  (params (Unit :type BP%20Unit%20Object%20Reference))
  (if (== Unit (Variables|Default|GetCurrent%20Unit))
    (Default|ClearStatefromTiles (Variables|/Game/2-Blueprints/Core/Player/BP_PlayerActions.BP_PlayerActions_C|GetBP_Grid (Variables|Default|GetBP_PlayerActions)) "NewEnumerator4")))