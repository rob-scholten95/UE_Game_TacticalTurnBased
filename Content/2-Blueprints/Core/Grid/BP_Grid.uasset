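; BP_Grid is a tile grid actor supporting square, hexagon and triangle shapes, storing each tile's type, transform and states.
; Construction spawns tiles, optionally sphere-tracing ground and BP_GridModifier actors for height and type.
; Child actors handle visuals and two pathfinders; tile edits update the visual and fire notifications.
; It maps world or cursor locations to indices and keeps a state-to-indices map for quick lookup.
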(fn ConstructionScript
  (Variables|Default|SetBP_Grid%20Visual (.AsBP%20Grid%20Visual (Utilities|Casting|CastToBP_GridVisual (Variables|/Script/Engine.ChildActorComponent|GetChildActor (Variables|Default|GetChildActor_GridVisual)))))
  (bind _output_get (Variables|Default|SetBP_GridPathFinding (.AsBP%20Grid%20Path%20Finding (Utilities|Casting|CastToBP_GridPathFinding (Variables|/Script/Engine.ChildActorComponent|GetChildActor (Variables|Default|GetChildActor_PathFinding))))))
  (Variables|/Game/2-Blueprints/Core/Grid/BP_GridPathFinding.BP_GridPathFinding_C|SetBP_Grid _output_get self)
  (bind _output_get_2 (Variables|Default|SetBP_GridPathFinding_Reachables (.AsBP%20Grid%20Path%20Finding (Utilities|Casting|CastToBP_GridPathFinding (Variables|/Script/Engine.ChildActorComponent|GetChildActor (Variables|Default|GetChildActor_PathFinding_Reachables))))))
  (Variables|/Game/2-Blueprints/Core/Grid/BP_GridPathFinding.BP_GridPathFinding_C|SetBP_Grid _output_get_2 self)
  (Grid|SpawnGrid (Transformation|GetActorLocation) (Variables|Default|GetTile%20Size) (Variables|Default|GetTile%20Count) (Variables|Default|GetGridShape) true))

(fn SpawnGrid
  (params (CenterLocation :type Vector) (TileSize :type Vector) (TileCount :type Int%20Point%20Structure) (ShapeType :type EN_GridShapes%20Enum :default "NewEnumerator0") (UseEnvironment :type Boolean))
  (Utilities|FlowControl|Sequence
    (:then_0
      ;[1 1 1] Storing Variables To Start Spawning the Grid
      (Variables|Default|SetCenter%20Location CenterLocation)
      (Variables|Default|SetTile%20Size TileSize)
      (Variables|Default|SetGridShape ShapeType)
      (Variables|Default|SetTile%20Count TileCount))
    (:then_1
      ;[1 1 1] Destroy the current visual grid and clear the data map
      (Grid|DestroyGrid))
    (:then_2
      ;[1 1 1] Initialize the new Visual grid
      (Default|InitializeGridVisual (Variables|Default|GetBP_Grid%20Visual) self))
    (:then_3
      ;[1 1 1] Calculating and Storing the Center of the grid and the Left Bottom corner
      (bind (_center _bottomleft_corner_) (Grid|CalculateCenterandBottomLeft))
      (Variables|Default|SetCenter%20Location _center)
      (Variables|Default|SetGridBottomLeftCornerLocation _bottomleft_corner_))
    (:then_4
      (for _index (range 0 (- (.x (Variables|Default|GetTile%20Count)) 1))
        (LocalVariables|SetX _index)
        (if (Utilities|Enum|NotEqual(Enum) (Variables|Default|GetGridShape) "NewEnumerator1")
          ;[1 1 1] Other Shapes For loop
          (for _index_2 (range 0 (- (.y (Variables|Default|GetTile%20Count)) 1))
            (LocalVariables|SetY _index_2)
            (LocalVariables|SetIndex (Utilities|Struct|MakeIntPoint (LocalVariables|GetX) (LocalVariables|GetY)))
            (LocalVariables|SetTileTransform (Math|Transform|MakeTransform (Grid|GetTileLocationfromGridIndex (LocalVariables|GetIndex)) (CallFunction|GetTileRotationfromGridIndex (LocalVariables|GetIndex)) (CallFunction|GetTileScalefromGridIndex (LocalVariables|GetIndex))))
            (if UseEnvironment
              (bind (_out_location _tiletype) (Trace|TraceforGround (.Location (Math|Transform|BreakTransform (LocalVariables|GetTileTransform)))))
              (GridTile|AddGridTile (Utilities|Struct|MakeSTR_TileData (LocalVariables|GetIndex) _tiletype (Math|Transform|MakeTransform _out_location (.Rotation (Math|Transform|BreakTransform (LocalVariables|GetTileTransform))) (.Scale (Math|Transform|BreakTransform (LocalVariables|GetTileTransform)))) "NewEnumerator0" 0))
              (else
                (GridTile|AddGridTile (Utilities|Struct|MakeSTR_TileData (LocalVariables|GetIndex) "NewEnumerator1" (LocalVariables|GetTileTransform) "NewEnumerator0" 0)))))
          (else
            ;[1 1 1] Hexagon For loop
            (for _index_3 (range (Math|Integer|SelectInt 0 1 (CallFunction|IsIntEven (LocalVariables|GetX))) (- (* (.y (Variables|Default|GetTile%20Count)) 2) 1))
              (LocalVariables|SetY _index_3)
              (Utilities|FlowControl|Sequence
                (:then_0
                  (LocalVariables|SetIndex (Utilities|Struct|MakeIntPoint (LocalVariables|GetX) (LocalVariables|GetY)))
                  (LocalVariables|SetTileTransform (Math|Transform|MakeTransform (Grid|GetTileLocationfromGridIndex (LocalVariables|GetIndex)) (CallFunction|GetTileRotationfromGridIndex (LocalVariables|GetIndex)) (CallFunction|GetTileScalefromGridIndex (LocalVariables|GetIndex))))
                  (if UseEnvironment
                    (bind (_out_location_2 _tiletype_2) (Trace|TraceforGround (.Location (Math|Transform|BreakTransform (LocalVariables|GetTileTransform)))))
                    (GridTile|AddGridTile (Utilities|Struct|MakeSTR_TileData (LocalVariables|GetIndex) _tiletype_2 (Math|Transform|MakeTransform _out_location_2 (.Rotation (Math|Transform|BreakTransform (LocalVariables|GetTileTransform))) (.Scale (Math|Transform|BreakTransform (LocalVariables|GetTileTransform)))) "NewEnumerator0" 0))
                    (else
                      (GridTile|AddGridTile (Utilities|Struct|MakeSTR_TileData (LocalVariables|GetIndex) "NewEnumerator1" (LocalVariables|GetTileTransform) "NewEnumerator0" 0)))))
                (:then_1
                  (Math|Integer|IncrementInt _index_3))))))))
    (:then_5
      (Default|CallOnGridGenerated))))

(fn GetCurrentShapeData
  (return (CallFunction|GetShapeData (Variables|Default|GetGridShape))))

(fn DestroyGrid
  ;[1 1 1] Clearing the Data of the Tiles
  (Utilities|Map|Clear (Variables|Default|GetGridTiles))
  ;[1 1 1] Destroying The visual of the grid
  (Default|DestroyGridVisual (Variables|Default|GetBP_Grid%20Visual))
  (Default|CallOnGridDestroyed))

(fn CalculateCenterandBottomLeft
  (bind _tile_count (Variables|Default|GetTile%20Count))
  (switch Utilities|FlowControl|Switch|SwitchonEN_GridShapes (Variables|Default|GetGridShape)
    (:NewEnumerator1
      ;[1 1 1] HEXAGON
      ;;[1 1 1] Snap Center Location to Tile size Adjusted to Hexagon
      (LocalVariables|SetC (CallFunction|SnaptoVectortoVector (Variables|Default|GetCenter%20Location) (* (Variables|Default|GetTile%20Size) "1.500000,1.000000,1.000000")))
      (return (LocalVariables|GetC) (- (LocalVariables|GetC) (CallFunction|SnaptoVectortoVector (Math|Conversions|ToVector(Vector2D) (* (/ (Variables|Default|GetTile%20Count) "(X=3.000000,Y=2.000000)") (Math|Conversions|ToVector2D(Vector) (Variables|Default|GetTile%20Size)))) (* (Variables|Default|GetTile%20Size) "1.500000,1.000000,1.000000")))))
    (:NewEnumerator2
      ;[1 1 1] SQUARE
      ;;[1 1 1] Snap Center Location to Tile Size Grid
      (LocalVariables|SetC (CallFunction|SnaptoVectortoVector (Variables|Default|GetCenter%20Location) (Variables|Default|GetTile%20Size)))
      (return (LocalVariables|GetC) (- (LocalVariables|GetC) (* (/ (- (Variables|Default|GetTile%20Count) (Math|Vector2D|MakeVector2D (Math|Float|SelectFloat 0.0 1.0 (CallFunction|IsIntEven (.x _tile_count))) (Math|Float|SelectFloat 0.0 1.0 (CallFunction|IsIntEven (.y _tile_count))))) 2.0) (Math|Conversions|ToVector2D(Vector) (Variables|Default|GetTile%20Size))))))
    (:NewEnumerator3
      ;[1 1 1] TRIANGLE
      ;;[1 1 1] Snap Center Location to Tile size Adjusted to Triangles
      (LocalVariables|SetC (CallFunction|SnaptoVectortoVector (Variables|Default|GetCenter%20Location) (* (Variables|Default|GetTile%20Size) "2.000000,1.000000,1.000000")))
      (return (LocalVariables|GetC) (- (LocalVariables|GetC) (CallFunction|SnaptoVectortoVector (Math|Conversions|ToVector(Vector2D) (* (/ (- (Variables|Default|GetTile%20Count) (Math|Vector2D|MakeVector2D 1.0 1.0)) "(X=2.000000,Y=4.000000)") (Math|Conversions|ToVector2D(Vector) (Variables|Default|GetTile%20Size)))) (* (Variables|Default|GetTile%20Size) "2.000000,1.000000,1.000000")))))))

(fn GetTileRotationfromGridIndex
  (params (GridIndex :type Int%20Point%20Structure))
  (if (Utilities|Enum|Equal(Enum) (Variables|Default|GetGridShape) "NewEnumerator3")
    (return (Math|Rotator|MakeRotator 0.0 0.0 (+ (Math|Float|SelectFloat 1.8e+02 0.0 (CallFunction|IsIntEven (.x GridIndex))) (Math|Float|SelectFloat 1.8e+02 0.0 (CallFunction|IsIntEven (.y GridIndex))))))
    (else
      (return "0, 0, 0"))))

(fn GetTileLocationfromGridIndex
  (params (GridIndex :type Int%20Point%20Structure))
  (return (+ (Variables|Default|GetGridBottomLeftCornerLocation) (* (Variables|Default|GetTile%20Size) (Math|Conversions|ToVector(Vector2D) (* GridIndex (Utilities|Select :Index (Variables|Default|GetGridShape) :NewEnumerator0 "" :NewEnumerator1 "(X=0.750000,Y=0.500000)" :NewEnumerator2 "(X=1.000000,Y=1.000000)" :NewEnumerator3 "(X=1.000000,Y=0.500000)")))))))

(fn TraceforGround
  (params (TileLocation :type Vector))
  (Variables|Default|SetRadius (/ (.x (Variables|Default|GetTile%20Size)) (Math|Float|SelectFloat 5.0 3.0 (Utilities|Enum|Equal(Enum) (Variables|Default|GetGridShape) "NewEnumerator3"))))
  ;[1 1 1] RAYCAST to find tiles with channel 'Ground'
  (bind _outhits (Collision|MultiSphereTraceByChannel (+ TileLocation "0.000000,0.000000,1000.000000") (- TileLocation "0.000000,0.000000,1000.000000") (Variables|Default|GetRadius) "TraceTypeQuery3" true 0 "None"))
  ;[1 1 1] Check if Something with channel "Ground" has been hit
  (if (> (Utilities|Array|Length _outhits) 0)
    (LocalVariables|SetIsHeightFound false)
    (LocalVariables|SetType "NewEnumerator1")
    (for _array_element _outhits
      (bind _asbp_grid_modifier (Utilities|Casting|CastToBP_GridModifier (.HitActor (Collision|BreakHitResult _array_element)))
        (:then
          (Utilities|IsValid _asbp_grid_modifier
            (:Is%20Valid
              (LocalVariables|SetType (Variables|/Game/2-Blueprints/Core/Grid/BP_GridModifier.BP_GridModifier_C|GetType _asbp_grid_modifier))
              (if (Variables|/Game/2-Blueprints/Core/Grid/BP_GridModifier.BP_GridModifier_C|GetUseForTileHeight _asbp_grid_modifier)
                (LocalVariables|SetIsHeightFound true)
                (LocalVariables|SetRetZ (- (.Z (Math|Vector|BreakVector (.Location (Collision|BreakHitResult _array_element)))) (Variables|Default|GetRadius)) :!label _label)))))
        (:CastFailed
          (if (not (LocalVariables|GetIsHeightFound))
            (goto _label)))))
    (return (Math|Vector|MakeVector (.x TileLocation) (.y TileLocation) (LocalVariables|GetRetZ)) (LocalVariables|GetType))
    (else
      ;[1 1 1] RETURN if nothing has been hit
      (return TileLocation "NewEnumerator0"))))

(fn GetTileIndexfromWorldLocation
  (params (Location :type Vector))
  ;[0 0 0] Convert to Worldspace to Gridspace
  (LocalVariables|SetLocationOnGrid (- Location (Variables|Default|GetGridBottomLeftCornerLocation)))
  ;[1 1 1] Comment
  (if (Utilities|Operators|NotEqual(!=) Location "-999.000000,-999.000000,-999.000000" 0.0001)
    (switch Utilities|FlowControl|Switch|SwitchonEN_GridShapes (Variables|Default|GetGridShape)
      (:NewEnumerator0
        (return (Utilities|Struct|MakeIntPoint -999 -999)))
      (:NewEnumerator1
        ;[0 0 0] Comment
        (LocalVariables|SetSnappedLocationOnGrid (Math|Conversions|ToVector2D(Vector) (CallFunction|SnaptoVectortoVector (* (LocalVariables|GetLocationOnGrid) "1.000000,2.000000,1.000000") (* (Variables|Default|GetTile%20Size) "0.750000,0.250000,1.000000"))))
        (LocalVariables|SetTempIndex (/ (LocalVariables|GetSnappedLocationOnGrid) (* (Math|Conversions|ToVector2D(Vector) (Variables|Default|GetTile%20Size)) "(X=0.750000,Y=1.000000)")))
        (if (CallFunction|IsFloatEven (.x (LocalVariables|GetTempIndex)))
          (return (Utilities|Struct|MakeIntPoint (Math|Float|Truncate (.x (LocalVariables|GetTempIndex))) (Math|Float|Truncate (* (Math|Float|Round (/ (.y (LocalVariables|GetTempIndex)) 2.0)) 2.0))))
          (else
            (return (Utilities|Struct|MakeIntPoint (Math|Float|Truncate (.x (LocalVariables|GetTempIndex))) (Math|Float|Truncate (+ (* (Math|Float|Floor (/ (.y (LocalVariables|GetTempIndex)) 2.0)) 2.0) 1.0)))))))
      (:NewEnumerator2
        ;[0 0 0] Comment
        (LocalVariables|SetSnappedLocationOnGrid (Math|Conversions|ToVector2D(Vector) (CallFunction|SnaptoVectortoVector (LocalVariables|GetLocationOnGrid) (Variables|Default|GetTile%20Size))))
        (return (Class|KismetMathLibrary|ToIntPoint(Vector2D) (/ (LocalVariables|GetSnappedLocationOnGrid) (Math|Conversions|ToVector2D(Vector) (Variables|Default|GetTile%20Size))))))
      (:NewEnumerator3
        ;[0 0 0] Comment
        (LocalVariables|SetSnappedLocationOnGrid (Math|Conversions|ToVector2D(Vector) (CallFunction|SnaptoVectortoVector (LocalVariables|GetLocationOnGrid) (/ (Variables|Default|GetTile%20Size) "1.000000,2.000000,1.000000"))))
        (return (Class|KismetMathLibrary|ToIntPoint(Vector2D) (* (/ (LocalVariables|GetSnappedLocationOnGrid) (Math|Conversions|ToVector2D(Vector) (Variables|Default|GetTile%20Size))) "(X=1.000000,Y=2.000000)")))))
    (else
      (return (Utilities|Struct|MakeIntPoint -999 -999)))))

(fn AddGridTile
  (params (Data :type STR%20Tile%20Data%20Structure))
  (Utilities|Map|Add (Variables|Default|GetGridTiles) (.index Data) Data)
  (Default|UpdateTileVisual (Variables|Default|GetBP_Grid%20Visual) (Utilities|Struct|MakeSTR_TileData (.index Data) (.tiletype Data) (.transform Data) (.tilestate Data) 0))
  (Default|CallOnTileDataUpdated (.index Data)))

(fn GetCursorLocationonGrid
  (params (PlayerIndex :type Integer))
  (bind _returnvalue (Game|GetPlayerController PlayerIndex))
  (bind _center_location (Variables|Default|GetCenter%20Location))
  (bind (_hitresult _returnvalue_2) (Game|Player|GetHitResultUnderCursorbyChannel _returnvalue "TraceTypeQuery3" false))
  (bind (_worldlocation _worlddirection) (Game|Player|ConvertMouseLocationToWorldSpace _returnvalue))
  (bind _returnvalue_3 (Class|KismetMathLibrary|MakePlanefromPointandNormal _center_location "0.000000,0.000000,1.000000"))
  (bind (_hitresult_2 _returnvalue_4) (Game|Player|GetHitResultUnderCursorbyChannel _returnvalue "TraceTypeQuery4" false))
  (bind _returnvalue_5 (* _worlddirection 9999.0))
  (bind _returnvalue_6 (+ _worldlocation _returnvalue_5))
  (bind (_t _intersection _returnvalue_7) (Class|KismetMathLibrary|LinePlaneIntersection _worldlocation _returnvalue_6 _returnvalue_3))
  (if _returnvalue_4
    (return (.Location (Collision|BreakHitResult _hitresult_2)))
    (elif _returnvalue_2
      (return (.Location (Collision|BreakHitResult _hitresult)))
      (elif _returnvalue_7
        (return _intersection)
        (else
          (return "-999.000000,-999.000000,-999.000000"))))))

(fn GetTileIndexUnderCursor
  (params (PlayerIndex :type Integer))
  (bind _location (Trace|GetCursorLocationonGrid PlayerIndex))
  (bind _index (CallFunction|GetTileIndexfromWorldLocation _location))
  (return _index))

(fn AddStatetoTile
  (params (Index :type Int%20Point%20Structure) (State :type EN_TileState%20Enum :default "NewEnumerator0"))
  (bind _gridtiles (Variables|Default|GetGridTiles))
  (bind (_value _returnvalue) (Utilities|Map|Find _gridtiles Index))
  (if _returnvalue
    (bind _output_get (LocalVariables|SetData _value))
    (bind _returnvalue_2 (Utilities|Array|AddUnique (.tilestate _output_get) State))
    (if (>= _returnvalue_2 0)
      (Utilities|Map|Add (Variables|Default|GetGridTiles) (.index (LocalVariables|GetData)) (LocalVariables|GetData))
      (bind _indexes (States|GetAllTileswithState State))
      (Utilities|Array|Add _indexes Index)
      (Utilities|Map|Add (Variables|Default|GetTileStateToIndexes) State (Utilities|Struct|MakeSTR_IntPointArray _indexes))
      (Default|UpdateTileVisual (Variables|Default|GetBP_Grid%20Visual) (LocalVariables|GetData))
      (Default|CallOnTileStateUpdated Index))))

(fn RemoveStatefromTile
  (params (Index :type Int%20Point%20Structure%20%28by%20ref%29) (TileState :type EN_TileState%20Enum :default "NewEnumerator0"))
  (bind _gridtiles (Variables|Default|GetGridTiles))
  (bind (_value _returnvalue) (Utilities|Map|Find _gridtiles Index))
  (if _returnvalue
    (bind _output_get (LocalVariables|SetData _value))
    (bind _returnvalue_2 (Utilities|Array|RemoveItem (.tilestate _output_get) TileState))
    (if _returnvalue_2
      (Utilities|Map|Add (Variables|Default|GetGridTiles) (.index (LocalVariables|GetData)) (LocalVariables|GetData))
      (bind _indexes (States|GetAllTileswithState TileState))
      (Utilities|Array|RemoveItem _indexes Index)
      (Utilities|Map|Add (Variables|Default|GetTileStateToIndexes) TileState (Utilities|Struct|MakeSTR_IntPointArray _indexes))
      (Default|UpdateTileVisual (Variables|Default|GetBP_Grid%20Visual) (LocalVariables|GetData))
      (Default|CallOnTileStateUpdated (.index (LocalVariables|GetData))))))

(fn IsIndexValid
  (params (Index :type Int%20Point%20Structure))
  (return (Utilities|Map|Contains (Variables|Default|GetGridTiles) Index)))

(fn GetTileScalefromGridIndex
  (params (Index :type Int%20Point%20Structure))
  (return (/ (Variables|Default|GetTile%20Size) (.meshsize (GridTile|GetCurrentShapeData)))))

(fn RemoveGridTile
  (params (Index :type Int%20Point%20Structure))
  (bind _returnvalue (Utilities|Map|Remove (Variables|Default|GetGridTiles) Index))
  (if _returnvalue
    (Default|UpdateTileVisual (Variables|Default|GetBP_Grid%20Visual) (Utilities|Struct|MakeSTR_TileData Index "NewEnumerator0" "0.000000,0.000000,0.000000|0.000000,0.000000,0.000000|1.000000,1.000000,1.000000" "NewEnumerator0" 0))
    (Default|CallOnTileDataUpdated Index)))

(fn GetAllTileswithState
  (params (State :type EN_TileState%20Enum :default "NewEnumerator0"))
  (return (.intpointarray (.Value (Utilities|Map|Find (Variables|Default|GetTileStateToIndexes) State)))))

(fn ClearStatefromTiles
  (params (State :type EN_TileState%20Enum :default "NewEnumerator0"))
  (bind _indexes (States|GetAllTileswithState State))
  (for _array_element _indexes
    (States|RemoveStatefromTile _array_element State)))

(fn IsTileWalkable
  (params (Index :type Int%20Point%20Structure))
  (return (CallFunction|IsTileWalkable (.TileType (Utilities|Struct|BreakSTR_TileData (.Value (Utilities|Map|Find (Variables|Default|GetGridTiles) Index)))))))