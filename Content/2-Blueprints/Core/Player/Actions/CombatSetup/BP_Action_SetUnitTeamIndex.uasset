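; Player action actor that assigns a team index to the unit on a selected grid tile, used in combat setup.
; Execute Action looks up the tile by index in the grid's tile map and, if a valid unit stands on it, passes that unit and the action's TeamIndex to the combat system's SetUnitTeamIndex.
; Grid and combat system are reached through the owning player actions object; the event graph holds only disabled default events.
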(event EventBeginPlay
  (|CallParentFunction) ; This node is disabled and will not be called.\nDrag off pins to build functionality.
)

(event Collision|EventActorBeginOverlap
  (params (OtherActor :type Actor%20Object%20Reference))
  (|CallParentFunction OtherActor) ; This node is disabled and will not be called.\nDrag off pins to build functionality.
)

(event EventTick
  (params (DeltaSeconds :type Float%20%28single-precision%29))
  (|CallParentFunction DeltaSeconds) ; This node is disabled and will not be called.\nDrag off pins to build functionality.
)

(fn ConstructionScript
  (|CallParentFunction))

(fn ExecuteAction
  (params (Index :type Int%20Point%20Structure))
  (bind _bp_playeractions (Variables|Default|GetBP_PlayerActions))
  (bind _bp_grid (Variables|/Game/2-Blueprints/Core/Player/BP_PlayerActions.BP_PlayerActions_C|GetBP_Grid _bp_playeractions))
  (bind _gridtiles (Variables|/Game/2-Blueprints/Core/Grid/BP_Grid.BP_Grid_C|GetGridTiles _bp_grid))
  (bind _value (Utilities|Map|Find _gridtiles Index))
  (bind _unitontile (Utilities|Struct|BreakSTR_TileData _value))
  (Utilities|IsValid _unitontile
    (:Is%20Valid
      (Default|SetUnitTeamIndex (Variables|/Game/2-Blueprints/Core/Player/BP_PlayerActions.BP_PlayerActions_C|GetBP_CombatSystem (Variables|Default|GetBP_PlayerActions)) _unitontile (Variables|Default|GetTeamIndex)))))