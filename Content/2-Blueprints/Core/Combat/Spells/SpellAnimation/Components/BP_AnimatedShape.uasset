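; BP_AnimatedShape is a spell animation actor that moves a colored mesh from an origin transform to a target transform.
; On BeginPlay it applies its mesh, material and color, then plays a timeline at a set rate.
; The timeline's alpha interpolates the transform, while its height curve and a fixed lift offset Z.
; On finish it fires OnShapeAnimationCompleted and destroys itself after a short delay.
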(event EventBeginPlay
  (Components|StaticMesh|SetStaticMesh (Variables|Default|GetAnimatedShape) (Variables|Default|GetMesh))
  (Rendering|Material|SetMaterial (Variables|Default|GetAnimatedShape) 0 (Variables|Default|GetMaterial))
  (Rendering|Material|SetVectorParameterValueonMaterials (Variables|Default|GetAnimatedShape) "Color" (Math|Conversions|ToVector(LinearColor) (Variables|Default|GetColor)))
  (Components|Timeline|SetPlayRate (Variables|Default|GetTimeline) (Variables|Default|GetPlay%20Rate))
  (bind (_direction _alpha _heightoffset) (Timeline|Timeline PlayFromStart)
    (:Update
      (Transformation|SetActorTransform (Math|Transform|MakeTransform (+ (.location (Math|Transform|Lerp(Transform) (Variables|Default|GetOriginTransform) (Variables|Default|GetTargetTransform) _alpha)) "0.000000,0.000000,100.000000" (Math|Vector|MakeVector 0.0 0.0 _heightoffset)) (.rotation (Math|Transform|Lerp(Transform) (Variables|Default|GetOriginTransform) (Variables|Default|GetTargetTransform) _alpha)) (.scale (Math|Transform|Lerp(Transform) (Variables|Default|GetOriginTransform) (Variables|Default|GetTargetTransform) _alpha)))))
    (:Finished
      (Default|CallOnShapeAnimationCompleted self)
      (Utilities|FlowControl|Delay 0.5)
      (Actor|DestroyActor))))

(event Collision|EventActorBeginOverlap
  (params (OtherActor :type Actor%20Object%20Reference)))

(event EventTick
  (params (DeltaSeconds :type Float%20%28single-precision%29)))

(fn ConstructionScript)