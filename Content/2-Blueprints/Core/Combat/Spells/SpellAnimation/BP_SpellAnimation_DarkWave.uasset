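; Spell animation actor for Dark Wave, showing a red-tinted, three-mesh effect at the spell's target tile.
; When played, it moves to the target tile, and a timeline drives the effect's scale and feeds opacity to a material parameter named None.
; From 0.2 seconds in, it reports a hit once for every attacked tile, then signals completion when the timeline finishes.
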(event EventBeginPlay
  (|CallParentFunction) ; This node is disabled and will not be called.\nDrag off pins to build functionality.
)

(event Collision|EventActorBeginOverlap
  (params (OtherActor :type Actor%20Object%20Reference)))

(event EventTick
  (params (DeltaSeconds :type Float%20%28single-precision%29)))

(event EventEventPlaySpellAnimation
  (Transformation|SetActorLocation (.location (CallFunction|GetTileTransform (Variables|Default|GetTargetIndex))) false false)
  (bind (_direction _opacity _scale) (Timeline|Timeline PlayFromStart)
    (:Update
      (Transformation|SetRelativeScale3D (Variables|Default|GetAnim) _scale)
      (Rendering|Material|SetScalarParameterValueonMaterials (Variables|Default|GetStaticMesh) "None" _opacity)
      (if (>= (Components|Timeline|GetPlaybackPosition (Variables|Default|GetTimeline)) 0.2)
        (Utilities|FlowControl|DoOnce false
          (:Completed
            (for _array_element (Variables|Default|GetAttackedIndexes)
              (Default|CallOnSpellAnimationHitTile self _array_element))))))
    (:Finished
      (CallFunction|EventCompleteSpellAnimation))))

(fn ConstructionScript
  (|CallParentFunction)
  (Rendering|Material|SetVectorParameterValueonMaterials (Variables|Default|GetStaticMesh1) "Color" (Math|Conversions|ToVector(LinearColor) "(R=0.895833,G=0.116943,B=0.063436,A=1.000000)"))
  (Rendering|Material|SetVectorParameterValueonMaterials (Variables|Default|GetStaticMesh2) "Color" (Math|Conversions|ToVector(LinearColor) "(R=0.421875,G=0.055072,B=0.029874,A=1.000000)"))
  (Rendering|Material|SetVectorParameterValueonMaterials (Variables|Default|GetStaticMesh) "Color" (Math|Conversions|ToVector(LinearColor) "(R=0.234375,G=0.030595,B=0.016598,A=1.000000)")))