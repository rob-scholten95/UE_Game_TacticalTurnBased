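; Player combat action that casts a selected spell from the selected grid tile onto a target tile.
; SetSpell loads the spell's cast and AOE data, then marks castable tiles with a grid tile state from the combat system's range query.
; Hovering a castable tile previews the AOE in a second state, or just that tile without a pattern.
; Executing delegates to the combat system and deselects the spell in the UI.
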(event EventBeginPlay
  (|CallParentFunction) ; This node is disabled and will not be called.\nDrag off pins to build functionality.
)

(event Collision|EventActorBeginOverlap
  (params (OtherActor :type Actor%20Object%20Reference))
  (|CallParentFunction OtherActor) ; This node is disabled and will not be called.\nDrag off pins to build functionality.
)

(event EventTick
  (params (DeltaSeconds :type Float%20%28single-precision%29))
  (|CallParentFunction DeltaSeconds) ; This node is disabled and will not be called.\nDrag off pins to build functionality.
)

(event EventEndPlay
  (params (EndPlayReason :type EEndPlayReason%20Enum :default "Destroyed"))
  (bind _bp_playeractions (Variables|Default|GetBP_PlayerActions))
  (bind _bp_grid (Variables|/Game/2-Blueprints/Core/Player/BP_PlayerActions.BP_PlayerActions_C|GetBP_Grid _bp_playeractions))
  (|CallParentFunction EndPlayReason)
  (Default|ClearStatefromTiles _bp_grid "NewEnumerator8")
  (Default|ClearStatefromTiles _bp_grid "NewEnumerator8"))

(fn ConstructionScript
  (|CallParentFunction))

(fn SetSpell
  (params (Spell :type EN_Spell%20Enum :default "NewEnumerator0"))
  (bind _bp_playeractions (Variables|Default|GetBP_PlayerActions))
  (bind _bp_grid (Variables|/Game/2-Blueprints/Core/Player/BP_PlayerActions.BP_PlayerActions_C|GetBP_Grid _bp_playeractions))
  (bind _output_get (Variables|Default|SetSpell Spell))
  (if (Utilities|Enum|NotEqual(Enum) _output_get "NewEnumerator0")
    (bind _spelldata (CallFunction|GetSpellDatafromSpell (Variables|Default|GetSpell)))
    (Variables|Default|SetCast (.Cast (Utilities|Struct|BreakSTR_SpellData _spelldata)))
    (Variables|Default|SetCastAOE (.AOE (Utilities|Struct|BreakSTR_SpellData _spelldata)))
    (CallFunction|ShowSpellRangePattern)
    (else
      (Default|ClearStatefromTiles _bp_grid "NewEnumerator8")
      (Default|ClearStatefromTiles _bp_grid "NewEnumerator9"))))

(fn ShowSpellRangePattern
  (bind _bp_playeractions (Variables|Default|GetBP_PlayerActions))
  (Utilities|FlowControl|Sequence
    (:then_0
      (Default|ClearStatefromTiles (Variables|/Game/2-Blueprints/Core/Player/BP_PlayerActions.BP_PlayerActions_C|GetBP_Grid (Variables|Default|GetBP_PlayerActions)) "NewEnumerator8")
      (bind _range_indexes (Default|GetSpellRange (Variables|/Game/2-Blueprints/Core/Player/BP_PlayerActions.BP_PlayerActions_C|GetBP_CombatSystem _bp_playeractions) (Variables|/Game/2-Blueprints/Core/Player/BP_PlayerActions.BP_PlayerActions_C|GetSelectedTileIndex _bp_playeractions) (Variables|Default|GetCast)))
      (for _array_element _range_indexes
        (Default|AddStatetoTile (Variables|/Game/2-Blueprints/Core/Player/BP_PlayerActions.BP_PlayerActions_C|GetBP_Grid (Variables|Default|GetBP_PlayerActions)) _array_element "NewEnumerator8")))
    (:then_1
      (CallFunction|ShowSpellRangePatternAOE))))

(fn ExecuteAction
  (params (Index :type Int%20Point%20Structure))
  (bind _bp_playeractions (Variables|Default|GetBP_PlayerActions))
  (bind _bp_playeractions_2 (Variables|Default|GetBP_PlayerActions))
  (bind _uw_combat (Variables|/Game/2-Blueprints/Core/Player/BP_PlayerActions.BP_PlayerActions_C|GetUW_Combat _bp_playeractions))
  (|CallParentFunction Index)
  (Default|CastSpell (Variables|/Game/2-Blueprints/Core/Player/BP_PlayerActions.BP_PlayerActions_C|GetBP_CombatSystem _bp_playeractions_2) (Variables|Default|GetSpell) (Variables|/Game/2-Blueprints/Core/Player/BP_PlayerActions.BP_PlayerActions_C|GetSelectedTileIndex _bp_playeractions_2) Index)
  (Utilities|IsValid _uw_combat
    (:Is%20Valid
      (Default|SetSelectedSpellfromIndex (Variables|/Game/2-Blueprints/Core/Combat/Widgets/UW_Combat.UW_Combat_C|GetUW_Button_ListSpells _uw_combat) -1))))

(fn ShowSpellRangePatternAOE
  (bind _bp_playeractions (Variables|Default|GetBP_PlayerActions))
  (Default|ClearStatefromTiles (Variables|/Game/2-Blueprints/Core/Player/BP_PlayerActions.BP_PlayerActions_C|GetBP_Grid (Variables|Default|GetBP_PlayerActions)) "NewEnumerator9")
  (if (Utilities|Array|ContainsItem (Utilities|Struct|BreakSTR_IntPointArray (.Value (Utilities|Map|Find (Variables|/Game/2-Blueprints/Core/Grid/BP_Grid.BP_Grid_C|GetTileStateToIndexes (Variables|/Game/2-Blueprints/Core/Player/BP_PlayerActions.BP_PlayerActions_C|GetBP_Grid (Variables|Default|GetBP_PlayerActions))) "NewEnumerator8"))) (Variables|/Game/2-Blueprints/Core/Player/BP_PlayerActions.BP_PlayerActions_C|GetHoveredTileIndex (Variables|Default|GetBP_PlayerActions)))
    (if (Utilities|Enum|NotEqual(Enum) (.RangePattern (Utilities|Struct|BreakSTR_SpellData_Cast (Variables|Default|GetCastAOE))) "NewEnumerator0")
      (bind _range_indexes (Default|GetSpellRange (Variables|/Game/2-Blueprints/Core/Player/BP_PlayerActions.BP_PlayerActions_C|GetBP_CombatSystem _bp_playeractions) (Variables|/Game/2-Blueprints/Core/Player/BP_PlayerActions.BP_PlayerActions_C|GetHoveredTileIndex _bp_playeractions) (Variables|Default|GetCastAOE)))
      (for _array_element _range_indexes
        (Default|AddStatetoTile (Variables|/Game/2-Blueprints/Core/Player/BP_PlayerActions.BP_PlayerActions_C|GetBP_Grid (Variables|Default|GetBP_PlayerActions)) _array_element "NewEnumerator9"))
      (else
        (Default|AddStatetoTile (Variables|/Game/2-Blueprints/Core/Player/BP_PlayerActions.BP_PlayerActions_C|GetBP_Grid (Variables|Default|GetBP_PlayerActions)) (Variables|/Game/2-Blueprints/Core/Player/BP_PlayerActions.BP_PlayerActions_C|GetHoveredTileIndex (Variables|Default|GetBP_PlayerActions)) "NewEnumerator9")))))

(fn ExecuteHoveredAction
  (params (Index :type Int%20Point%20Structure))
  (|CallParentFunction Index)
  (CallFunction|ShowSpellRangePatternAOE))