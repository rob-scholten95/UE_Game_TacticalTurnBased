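; Animated wind gust actor that serves as a visual component of a spell animation.
; On BeginPlay a timeline at a configurable play rate lerps the actor from origin to target transform and drives the material's opacity.
; Partway through it fires the shape-animation-completed event once, ahead of the timeline's end, then destroys itself shortly after finishing.
; The construction script gives both material slots translucent green dynamic instances with randomized brightness.
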(event EventBeginPlay
  (Components|Timeline|SetPlayRate (Variables|Default|GetTimeline) (Variables|Default|GetPlay%20Rate))
  (bind (_direction _transformalpha _opacity) (Timeline|Timeline PlayFromStart)
    (:Update
      (Transformation|SetActorTransform (Math|Transform|Lerp(Transform) (Variables|Default|GetOriginTransform) (Variables|Default|GetTargetTransform) _transformalpha))
      (Rendering|Material|SetScalarParameterValueonMaterials (Variables|Default|GetAnimatedWindGust) "Alpha" _opacity)
      (if (>= (Components|Timeline|GetPlaybackPosition (Variables|Default|GetTimeline)) 0.35)
        (Utilities|FlowControl|DoOnce false
          (:Completed
            (Default|CallOnShapeAnimationCompleted self)))))
    (:Finished
      (Utilities|FlowControl|Delay 0.5)
      (Actor|DestroyActor))))

(event Collision|EventActorBeginOverlap
  (params (OtherActor :type Actor%20Object%20Reference)))

(event EventTick
  (params (DeltaSeconds :type Float%20%28single-precision%29)))

(fn ConstructionScript
  (bind _returnvalue (Rendering|Material|CreateDynamicMaterialInstance (Variables|Default|GetAnimatedWindGust) 0 "/Game/4-Assets/Materials/M_TranslucentColor.M_TranslucentColor" "None" :!class /Script/Engine.PrimitiveComponent))
  (Rendering|Material|SetVectorParameterValue _returnvalue "Color" (* "(R=0.249758,G=0.968750,B=0.187810,A=1.000000)" (Math|Random|RandomFloatinRange 0.8 1.5)) :!class /Script/Engine.MaterialInstanceDynamic)
  (bind _returnvalue_2 (Rendering|Material|CreateDynamicMaterialInstance (Variables|Default|GetAnimatedWindGust) 1 "/Game/4-Assets/Materials/M_TranslucentColor.M_TranslucentColor" "None" :!class /Script/Engine.PrimitiveComponent))
  (Rendering|Material|SetVectorParameterValue _returnvalue_2 "Color" (* "(R=0.010417,G=1.000000,B=0.024235,A=1.000000)" (Math|Random|RandomFloatinRange 0.8 1.5)) :!class /Script/Engine.MaterialInstanceDynamic))