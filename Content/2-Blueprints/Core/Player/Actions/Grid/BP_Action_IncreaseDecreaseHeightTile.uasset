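; Player grid action that raises or lowers the tile at a given index, derived from a parent action class.
; When the index is valid, it looks up the tile data on the grid and re-adds it via AddGridTile with its Z location shifted by a fixed step.
; The Increase flag picks the direction, with true applying the negative offset; all other tile data is preserved.
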(fn ConstructionScript
  (|CallParentFunction))

(fn ExecuteAction
  (params (Index :type Int%20Point%20Structure))
  (if (Default|IsIndexValid (Variables|/Game/2-Blueprints/Core/Player/BP_PlayerActions.BP_PlayerActions_C|GetBP_Grid (Variables|Default|GetBP_PlayerActions)) Index)
    (LocalVariables|SetData (.Value (Utilities|Map|Find (Variables|/Game/2-Blueprints/Core/Grid/BP_Grid.BP_Grid_C|GetGridTiles (Variables|/Game/2-Blueprints/Core/Player/BP_PlayerActions.BP_PlayerActions_C|GetBP_Grid (Variables|Default|GetBP_PlayerActions))) Index)))
    (Default|AddGridTile (Variables|/Game/2-Blueprints/Core/Player/BP_PlayerActions.BP_PlayerActions_C|GetBP_Grid (Variables|Default|GetBP_PlayerActions)) (Utilities|Struct|MakeSTR_TileData (.index (LocalVariables|GetData)) (.tiletype (LocalVariables|GetData)) (Math|Transform|MakeTransform (+ (.Location (Math|Transform|BreakTransform (.transform (LocalVariables|GetData)))) (Math|Vector|MakeVector 0.0 0.0 (select (Variables|Default|GetIncrease) -3e+01 3e+01))) (.Rotation (Math|Transform|BreakTransform (.transform (LocalVariables|GetData)))) (.Scale (Math|Transform|BreakTransform (.transform (LocalVariables|GetData))))) (.tilestate (LocalVariables|GetData)) (.unitontile (LocalVariables|GetData))))))