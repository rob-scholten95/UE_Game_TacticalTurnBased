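; Spell animation actor that flies a long-range arrow from an origin tile to a target tile.
; On play it faces the target using the tile indices, then a timeline drives position along a lerp with added height, plus the Anim component's pitch and scale.
; The hit event for the target tile fires through a DoOnce once playback passes a fixed time, and the timeline's end completes the animation.
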(event EventBeginPlay
  (|CallParentFunction) ; This node is disabled and will not be called.\nDrag off pins to build functionality.
)

(event Collision|EventActorBeginOverlap
  (params (OtherActor :type Actor%20Object%20Reference)))

(event EventTick
  (params (DeltaSeconds :type Float%20%28single-precision%29)))

(event EventEventPlaySpellAnimation
  (Transformation|SetActorLocationAndRotation (.location (CallFunction|GetTileTransform (Variables|Default|GetOriginIndex))) (Math|Rotator|FindLookatRotation (Math|Conversions|ToVector(Vector2D) (Math|Conversions|ToVector2D(IntPoint) (Variables|Default|GetOriginIndex))) (Math|Conversions|ToVector(Vector2D) (Math|Conversions|ToVector2D(IntPoint) (Variables|Default|GetTargetIndex)))))
  (bind (_direction _actorlocationalpha _rotationy _scale _locationz) (Timeline|Timeline PlayFromStart)
    (:Update
      (Transformation|SetActorLocation (+ (Math|Vector|Lerp(Vector) (.location (CallFunction|GetTileTransform (Variables|Default|GetOriginIndex))) (.location (CallFunction|GetTileTransform (Variables|Default|GetTargetIndex))) _actorlocationalpha) (Math|Vector|MakeVector 0.0 0.0 _locationz)) false false)
      (Transformation|SetRelativeRotation (Variables|Default|GetAnim) (Math|Rotator|MakeRotator 0.0 _rotationy 0.0) false false)
      (Transformation|SetRelativeScale3D (Variables|Default|GetAnim) (Math|Conversions|ToVector(Float) _scale))
      (if (>= (Components|Timeline|GetPlaybackPosition (Variables|Default|GetTimeline)) 0.6)
        (Utilities|FlowControl|DoOnce false
          (:Completed
            (Default|CallOnSpellAnimationHitTile self (Variables|Default|GetTargetIndex))))))
    (:Finished
      (CallFunction|EventCompleteSpellAnimation))))

(fn ConstructionScript
  (|CallParentFunction))