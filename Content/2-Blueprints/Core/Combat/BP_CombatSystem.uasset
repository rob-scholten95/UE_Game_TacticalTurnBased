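; Turn-based grid combat manager that tracks units and teams, cycles turns through living units and signals combat start, finish and end.
; Keeps tile occupancy synced with BPGrid, removing units left on invalid tiles, and charges movement points by path cost.
; Spells filter pattern ranges by walkability and optional offset line-of-sight traces, then apply one random HP roll across the area.
; Deaths during combat trigger a surviving-team check to declare a winner.
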(event EventBeginPlay
  (bind _bp_grid (Variables|Default|GetBP_Grid))
  (EventDispatchers|BindEventtoOnGridGenerated _bp_grid (EventDispatchers|CreateEvent :!event OnGridGenerated))
  (EventDispatchers|BindEventtoOnTileDataUpdated _bp_grid (EventDispatchers|CreateEvent :!event OnTileDataUpdated)))

(event Collision|EventActorBeginOverlap
  (params (OtherActor :type Actor%20Object%20Reference)))

(event EventTick
  (params (DeltaSeconds :type Float%20%28single-precision%29)))

(fn ConstructionScript)

(fn AddUnittoCombat
  (params (Unit :type BP%20Unit%20Object%20Reference) (Index :type Int%20Point%20Structure) (TeamIndex :type Integer))
  (Utilities|Array|Add (Variables|Default|GetUnitsInCombat) Unit)
  (Default|SetGrid Unit (Variables|Default|GetBP_Grid))
  (Units|SetUnitIndexonGrid Unit Index false true)
  (EventDispatchers|BindEventtoOnUnitReachedNewTile Unit (EventDispatchers|CreateEvent :!event OnUnitReachedNewTile))
  (Team|SetUnitTeamIndex Unit TeamIndex))

(fn RemoveUnitfromCombat
  (params (Unit :type BP%20Unit%20Object%20Reference) (DestroyUnit :type Boolean))
  (Utilities|Array|RemoveItem (Variables|Default|GetUnitsInCombat) Unit)
  (Units|SetUnitIndexonGrid Unit (Utilities|Struct|MakeIntPoint -999 -999) false true)
  (Team|SetUnitTeamIndex Unit -1)
  (if DestroyUnit
    (Actor|DestroyActor Unit)))

(fn SetUnitIndexonGrid
  (params (Unit :type BP%20Unit%20Object%20Reference) (Index :type Int%20Point%20Structure) (Force :type Boolean) (Snap%20Location :type Boolean))
  (bind _bp_grid (Variables|Default|GetBP_Grid))
  (bind _gridtiles (Variables|/Game/2-Blueprints/Core/Grid/BP_Grid.BP_Grid_C|GetGridTiles _bp_grid))
  (bind (_value _returnvalue) (Utilities|Map|Find _gridtiles Index))
  (Utilities|FlowControl|Sequence
    (:then_0
      (if (or (!= (Variables|/Game/2-Blueprints/Core/Units/BP_Unit.BP_Unit_C|GetIndex Unit) Index) Force)
        (Utilities|FlowControl|Sequence
          (:then_0
            (bind _output_get (LocalVariables|SetPrevious%20Tile (.Value (Utilities|Map|Find (Variables|/Game/2-Blueprints/Core/Grid/BP_Grid.BP_Grid_C|GetGridTiles (Variables|Default|GetBP_Grid)) (Variables|/Game/2-Blueprints/Core/Units/BP_Unit.BP_Unit_C|GetIndex Unit)))))
            (if (== (.UnitOnTile (Utilities|Struct|BreakSTR_TileData _output_get)) Unit)
              (bind _structout (Utilities|Struct|SetmembersinSTR_TileData (LocalVariables|GetPrevious%20Tile)))
              (Utilities|Map|Add (Variables|/Game/2-Blueprints/Core/Grid/BP_Grid.BP_Grid_C|GetGridTiles (Variables|Default|GetBP_Grid)) (Utilities|Struct|BreakSTR_TileData _structout) _structout)))
          (:then_1
            (Default|SetGridIndex Unit Index)
            (if (!= Index (Utilities|Struct|MakeIntPoint -999 -999))
              (bind _structout_2 (Utilities|Struct|SetmembersinSTR_TileData (.Value (Utilities|Map|Find (Variables|/Game/2-Blueprints/Core/Grid/BP_Grid.BP_Grid_C|GetGridTiles (Variables|Default|GetBP_Grid)) Index)) Unit))
              (Utilities|Map|Add (Variables|/Game/2-Blueprints/Core/Grid/BP_Grid.BP_Grid_C|GetGridTiles (Variables|Default|GetBP_Grid)) (Utilities|Struct|BreakSTR_TileData _structout_2) _structout_2)))
          (:then_2
            (Default|CallOnUnitGridIndexChanged Unit)))))
    (:then_1
      (if Snap%20Location
        (Transformation|SetActorLocation Unit (select _returnvalue (.Location (Math|Transform|BreakTransform (.Transform (Utilities|Struct|BreakSTR_TileData _value)))) "-99999.000000,-99999.000000,-99999.000000") false false)))))

(fn OnGridGenerated
  (bind _output_get (LocalVariables|SetCopyOfUnitsInCombat (Variables|Default|GetUnitsInCombat)))
  (for _array_element _output_get
    (if (Utilities|Array|ContainsItem (.ValidTileTypes (Utilities|Struct|BreakSTR_UnitData_Stats (.Stats (Utilities|Struct|BreakSTR_UnitData (Variables|/Game/2-Blueprints/Core/Units/BP_Unit.BP_Unit_C|GetUnitData _array_element))))) (.tiletype (.Value (Utilities|Map|Find (Variables|/Game/2-Blueprints/Core/Grid/BP_Grid.BP_Grid_C|GetGridTiles (Variables|Default|GetBP_Grid)) (Variables|/Game/2-Blueprints/Core/Units/BP_Unit.BP_Unit_C|GetIndex _array_element)))))
      (Units|SetUnitIndexonGrid :Unit _array_element :Force true)
      (else
        (Units|RemoveUnitfromCombat _array_element true)))))

(fn OnTileDataUpdated
  (params (Index :type Int%20Point%20Structure))
  (bind _output_get (LocalVariables|SetCopyOfUnitsInCombat (Variables|Default|GetUnitsInCombat)))
  (bind _array_element (Utilities|Array|ForEachLoopwithBreak _output_get :!label _label)
    (:LoopBody
      (if (Class|KismetMathLibrary|EqualIntPointIntPoint Index (Variables|/Game/2-Blueprints/Core/Units/BP_Unit.BP_Unit_C|GetIndex _array_element))
        (if (Utilities|Array|ContainsItem (.ValidTileTypes (Utilities|Struct|BreakSTR_UnitData_Stats (.Stats (Utilities|Struct|BreakSTR_UnitData (Variables|/Game/2-Blueprints/Core/Units/BP_Unit.BP_Unit_C|GetUnitData _array_element))))) (.tiletype (.Value (Utilities|Map|Find (Variables|/Game/2-Blueprints/Core/Grid/BP_Grid.BP_Grid_C|GetGridTiles (Variables|Default|GetBP_Grid)) (Variables|/Game/2-Blueprints/Core/Units/BP_Unit.BP_Unit_C|GetIndex _array_element)))))
          (Units|SetUnitIndexonGrid _array_element (Variables|/Game/2-Blueprints/Core/Units/BP_Unit.BP_Unit_C|GetIndex _array_element) false true)
          (goto _label Break)
          (else
            (Units|RemoveUnitfromCombat _array_element true)
            (goto _label Break)))))))

(fn OnUnitReachedNewTile
  (params (Unit :type BP%20Unit%20Object%20Reference) (Index :type Int%20Point%20Structure))
  (Game|SpawnActorfromClass "/Game/2-Blueprints/Core/Units/Widget/BP_AnimatedNumber.BP_AnimatedNumber_C" (Math|Transform|MakeTransform (Transformation|GetActorLocation Unit) "0, 0, 0" "1.000000,1.000000,1.000000") "Undefined" "MultiplyWithRoot" 0 (- 0 (CallFunction|GetTileTypeCost (.TileType (Utilities|Struct|BreakSTR_TileData (.Value (Utilities|Map|Find (Variables|/Game/2-Blueprints/Core/Grid/BP_Grid.BP_Grid_C|GetGridTiles (Variables|Default|GetBP_Grid)) Index)))))) "NewEnumerator1" 0))

(fn CastSpell
  (params (Spell :type EN_Spell%20Enum :default "NewEnumerator0") (OriginIndex :type Int%20Point%20Structure) (TargetIndex :type Int%20Point%20Structure))
  (bind _bp_grid (Variables|Default|GetBP_Grid))
  (bind _bp_grid_2 (Variables|Default|GetBP_Grid))
  (bind _gridtiles (Variables|/Game/2-Blueprints/Core/Grid/BP_Grid.BP_Grid_C|GetGridTiles _bp_grid))
  (bind _gridtiles_2 (Variables|/Game/2-Blueprints/Core/Grid/BP_Grid.BP_Grid_C|GetGridTiles _bp_grid_2))
  (bind _value (Utilities|Map|Find _gridtiles_2 OriginIndex))
  (bind _value_2 (Utilities|Map|Find _gridtiles OriginIndex))
  (bind _unitontile (Utilities|Struct|BreakSTR_TileData _value))
  (bind _unitontile_2 (Utilities|Struct|BreakSTR_TileData _value_2))
  (bind _spelldata (CallFunction|GetSpellDatafromSpell Spell))
  (LocalVariables|SetData _spelldata)
  (Utilities|IsValid _unitontile_2
    (:Is%20Valid
      (bind _can_cast (Default|CanCastSpell _unitontile_2 (LocalVariables|GetData)))
      (if _can_cast
        (bind _range_indexes (Spells|GetSpellRange OriginIndex (.Cast (Utilities|Struct|BreakSTR_SpellData (LocalVariables|GetData))) :!label _label))
        (bind _output_get (LocalVariables|SetAttackedIndexes _range_indexes))
        (if (Utilities|Array|ContainsItem _output_get TargetIndex)
          (if (Utilities|Enum|Equal(Enum) (.RangePattern (Utilities|Struct|BreakSTR_SpellData_Cast (.AOE (Utilities|Struct|BreakSTR_SpellData (LocalVariables|GetData))))) "NewEnumerator0")
            (LocalVariables|SetAttackedIndexes (Utilities|Array|MakeArray TargetIndex))
            (else
              (bind _range_indexes_2 (Spells|GetSpellRange TargetIndex (.AOE (Utilities|Struct|BreakSTR_SpellData (LocalVariables|GetData)))))
              (LocalVariables|SetAttackedIndexes _range_indexes_2)))
          (bind _returnvalue (Game|SpawnActorfromClass (.Animation (Utilities|Struct|BreakSTR_SpellData_Assets (.Assets (Utilities|Struct|BreakSTR_SpellData (LocalVariables|GetData))))) (Math|Transform|MakeTransform "0, 0, 0" "0, 0, 0" "1.000000,1.000000,1.000000") "AlwaysSpawn" "MultiplyWithRoot" 0 (Variables|Default|GetBP_Grid) OriginIndex (LocalVariables|GetAttackedIndexes) TargetIndex 0))
          (LocalVariables|SetSpellAnimation _returnvalue)
          (Utilities|FlowControl|Sequence
            (:then_0
              (Utilities|IsValid _unitontile
                (:Is%20Valid
                  (Default|UnitCastSpell _unitontile TargetIndex (LocalVariables|GetData)))))
            (:then_1
              (Variables|Default|SetSTR%20Spell%20Data%20Impact%20Real (Utilities|Struct|MakeSTR_SpellData_Impact_Real (CallFunction|MinMaxRandom (Utilities|Struct|BreakSTR_SpellData_Impact (.Impact (Utilities|Struct|BreakSTR_SpellData (LocalVariables|GetData)))))))
              (for _array_element (LocalVariables|GetAttackedIndexes)
                (bind _output_get_2 (LocalVariables|SetUnit (Utilities|Struct|BreakSTR_TileData (.Value (Utilities|Map|Find (Variables|/Game/2-Blueprints/Core/Grid/BP_Grid.BP_Grid_C|GetGridTiles (Variables|Default|GetBP_Grid)) _array_element)))))
                (Utilities|IsValid _output_get_2
                  (:Is%20Valid
                    (if (Default|IsAlive _output_get_2)
                      (Default|UnitHitbySpell _output_get_2 (Variables|Default|GetSTR%20Spell%20Data%20Impact%20Real) (LocalVariables|GetSpellAnimation))
                      (if (not (Default|IsAlive (LocalVariables|GetUnit)))
                        (CallFunction|ProcessUnitDeath (LocalVariables|GetUnit))
                        (if (Variables|Default|GetIsFinishingCombat)
                          (return))))))))))))
    (:Is%20Not%20Valid
      (goto _label))))

(fn GetSpellRange
  (params (OriginIndex :type Int%20Point%20Structure) (Cast :type STR%20Spell%20Data%20Cast%20Structure))
  (bind (_rangepattern _rangeminmax _lineofsight) (Utilities|Struct|BreakSTR_SpellData_Cast Cast))
  (bind _rangeindexes (CallFunction|GetIndexesfromPatternandRange OriginIndex (Variables|/Game/2-Blueprints/Core/Grid/BP_Grid.BP_Grid_C|GetGridShape (Variables|Default|GetBP_Grid)) _rangepattern _rangeminmax))
  (bind _indexeswithlineofsight (Spells|RemoveNotWalkableIndexes _rangeindexes))
  (if (.RequireLineOfSight (Utilities|Struct|BreakSTR_SpellData_LineOfSight _lineofsight))
    (bind _indexeswithlineofsight_2 (Spells|RemoveIndexesWithoutLOS OriginIndex _indexeswithlineofsight Cast))
    (return _indexeswithlineofsight_2)
    (else
      (return _indexeswithlineofsight))))

(fn HasLineOfSight
  (params (OriginIndex :type Int%20Point%20Structure) (TargetIndex :type Int%20Point%20Structure) (Cast :type STR%20Spell%20Data%20Cast%20Structure))
  (bind _bp_grid (Variables|Default|GetBP_Grid))
  (bind _bp_grid_2 (Variables|Default|GetBP_Grid))
  (bind _lineofsight (Utilities|Struct|BreakSTR_SpellData_Cast Cast))
  (bind _lineofsight_2 (Utilities|Struct|BreakSTR_SpellData_Cast Cast))
  (bind _gridtiles (Variables|/Game/2-Blueprints/Core/Grid/BP_Grid.BP_Grid_C|GetGridTiles _bp_grid))
  (bind _tile_size (Variables|/Game/2-Blueprints/Core/Grid/BP_Grid.BP_Grid_C|GetTile%20Size _bp_grid_2))
  (bind _returnvalue (Math|Vector|MakeVector 0.0 0.0 (.height _lineofsight)))
  (bind _returnvalue_2 (* _tile_size (.offset _lineofsight_2)))
  (LocalVariables|SetOriginTile (.Value (Utilities|Map|Find _gridtiles OriginIndex)))
  (LocalVariables|SetTargetTile (.Value (Utilities|Map|Find _gridtiles TargetIndex)))
  (LocalVariables|SetStart (+ (.location (.Transform (Utilities|Struct|BreakSTR_TileData (LocalVariables|GetOriginTile)))) _returnvalue))
  (LocalVariables|SetEnd (+ _returnvalue (.location (.Transform (Utilities|Struct|BreakSTR_TileData (LocalVariables|GetTargetTile))))))
  (for _array_element (Utilities|Array|MakeArray (Math|Vector2D|MakeVector2D (.x _returnvalue_2) 0.0) (Math|Vector2D|MakeVector2D (- 0.0 (.x _returnvalue_2)) 0.0) (Math|Vector2D|MakeVector2D 0.0 (.y _returnvalue_2)) (Math|Vector2D|MakeVector2D 0.0 (- 0.0 (.z _returnvalue_2))))
    (bind _returnvalue_3 (Collision|LineTraceByChannel (+ (LocalVariables|GetStart) _array_element) (LocalVariables|GetEnd) "TraceTypeQuery6" false (Utilities|Array|MakeArray (Utilities|Struct|BreakSTR_TileData (LocalVariables|GetOriginTile)) (Utilities|Struct|BreakSTR_TileData (LocalVariables|GetTargetTile))) (select (.drawdebuglines (Utilities|Struct|BreakSTR_SpellData_Cast Cast)) "ForDuration" "None")))
    (if (not _returnvalue_3)
      (return true)))
  (return false))

(fn RemoveIndexesWithoutLOS
  (params (Origin%20Index :type Int%20Point%20Structure) (Indexes :type Array%20of%20Int%20Point%20Structures) (Cast :type STR%20Spell%20Data%20Cast%20Structure))
  (for _array_element Indexes
    (if (Spells|HasLineOfSight Origin%20Index _array_element Cast)
      (Utilities|Array|Add (LocalVariables|Getret) _array_element)))
  (return (LocalVariables|Getret)))

(fn RemoveNotWalkableIndexes
  (params (Indexes :type Array%20of%20Int%20Point%20Structures))
  (for _array_element Indexes
    (if (Default|IsTileWalkable (Variables|Default|GetBP_Grid) _array_element)
      (Utilities|Array|Add (LocalVariables|Getret) _array_element)))
  (return (LocalVariables|Getret)))

(fn SetUnitTeamIndex
  (params (Unit :type BP%20Unit%20Object%20Reference) (TeamIndex :type Integer))
  (Utilities|FlowControl|Sequence
    (:then_0
      (if (!= (Variables|/Game/2-Blueprints/Core/Units/BP_Unit.BP_Unit_C|GetTeamIndex Unit) -1)
        (bind _output_get (LocalVariables|SetUnitSet (.unitset (.Value (Utilities|Map|Find (Variables|Default|GetUnitTeams) (Variables|/Game/2-Blueprints/Core/Units/BP_Unit.BP_Unit_C|GetTeamIndex Unit))))))
        (Utilities|Set|Remove _output_get Unit)
        (if (> (Utilities|Set|Length (LocalVariables|GetUnitSet)) 0)
          (Utilities|Map|Add (Variables|Default|GetUnitTeams) (Variables|/Game/2-Blueprints/Core/Units/BP_Unit.BP_Unit_C|GetTeamIndex Unit) (Utilities|Struct|MakeSTR_UnitSet (LocalVariables|GetUnitSet)))
          (else
            (Utilities|Map|Remove (Variables|Default|GetUnitTeams) (Variables|/Game/2-Blueprints/Core/Units/BP_Unit.BP_Unit_C|GetTeamIndex Unit))))))
    (:then_1
      (if (!= TeamIndex -1)
        (bind _output_get_2 (LocalVariables|SetUnitSet (.unitset (.Value (Utilities|Map|Find (Variables|Default|GetUnitTeams) TeamIndex)))))
        (Utilities|Set|Add _output_get_2 Unit)
        (Utilities|Map|Add (Variables|Default|GetUnitTeams) TeamIndex (Utilities|Struct|MakeSTR_UnitSet (LocalVariables|GetUnitSet)))))
    (:then_2
      (Default|SetTeamIndex Unit TeamIndex)
      (Default|CallOnUnitTeamsChanged))))

(fn CanStartCombat
  (bind _unitsincombat (Variables|Default|GetUnitsInCombat))
  (bind _unitteams (Variables|Default|GetUnitTeams))
  (bind _isincombat (Variables|Default|GetIsInCombat))
  (bind _returnvalue (Utilities|Array|Length _unitsincombat))
  (bind _returnvalue_2 (Utilities|Map|Length _unitteams))
  (bind _returnvalue_3 (not _isincombat))
  (bind _returnvalue_4 (>= _returnvalue_2 2))
  (bind _returnvalue_5 (>= _returnvalue 2))
  (return (Math|Boolean|ANDBoolean _returnvalue_5 _returnvalue_4 _returnvalue_3) _returnvalue_5 _returnvalue_4 _returnvalue_3))

(fn StartCombat
  (Variables|Default|SetIsInCombat true)
  (for _array_element (Variables|Default|GetUnitsInCombat)
    (Default|CombatStarted _array_element))
  (Default|CallOnCombatStarted)
  (Variables|Default|SetCurrentUnit 0)
  (CallFunction|NextUnit))

(fn EndCombat
  (Variables|Default|SetIsInCombat false)
  (Variables|Default|SetIsFinishingCombat false)
  (Variables|Default|SetCurrentUnit 0)
  (for _array_element (Variables|Default|GetUnitsInCombat)
    (Default|CombatEnded _array_element))
  (Default|CallOnCombatEnded))

(fn NextUnit
  (Utilities|FlowControl|Sequence
    (:then_0
      (Utilities|IsValid (Variables|Default|GetCurrentUnit)
        (:Is%20Valid
          (Default|TurnEnded (Variables|Default|GetCurrentUnit))
          (Default|CallOnUnitTurnEnded (Variables|Default|GetCurrentUnit)))))
    (:then_1
      (LocalVariables|SetCurrent%20Index (Utilities|Array|FindItem (Variables|Default|GetUnitsInCombat) (Variables|Default|GetCurrentUnit)))
      (while (not (Utilities|IsValid (LocalVariables|GetNextLivingUnit)))
        (LocalVariables|SetCurrent%20Index (Math|Integer|%(Integer) (+ (LocalVariables|GetCurrent%20Index) 1) (Utilities|Array|Length (Variables|Default|GetUnitsInCombat))))
        (if (Default|IsAlive (Utilities|Array|Get(acopy) (Variables|Default|GetUnitsInCombat) (LocalVariables|GetCurrent%20Index)))
          (LocalVariables|SetNextLivingUnit (Utilities|Array|Get(acopy) (Variables|Default|GetUnitsInCombat) (LocalVariables|GetCurrent%20Index)))))
      (bind _output_get (Variables|Default|SetCurrentUnit (LocalVariables|GetNextLivingUnit)))
      (Default|TurnStarted _output_get)
      (Default|CallOnUnitTurnStarted (Variables|Default|GetCurrentUnit)))))

(fn MoveUnit
  (params (Unit :type BP%20Unit%20Object%20Reference) (Path :type Array%20of%20Int%20Point%20Structures))
  (if (Utilities|Array|IsNotEmpty Path)
    (Default|FollowPath Unit Path)
    (bind _cost (Default|GetPathCost (Variables|/Game/2-Blueprints/Core/Grid/BP_Grid.BP_Grid_C|GetBP_GridPathFinding (Variables|Default|GetBP_Grid)) Path))
    (Default|ModifyCurrentMP Unit (- 0 _cost) false)
    (Units|SetUnitIndexonGrid Unit (Utilities|Array|Get(acopy) Path (Utilities|Array|LastIndex Path)) false false)))

(fn ProcessUnitDeath
  (params (Unit :type BP%20Unit%20Object%20Reference))
  (bind _teamsalive (LocalVariables|GetTeamsAlive))
  (if (Variables|Default|GetIsInCombat)
    (Variables|/Game/2-Blueprints/Core/Units/BP_Unit.BP_Unit_C|SetIndexToRememberForSpellImpact Unit (Variables|/Game/2-Blueprints/Core/Units/BP_Unit.BP_Unit_C|GetIndex Unit))
    (Units|SetUnitIndexonGrid 0 (Utilities|Struct|MakeIntPoint -999 -999) false true)
    (Default|EventHideUnitAfterSeconds Unit)
    (bind _keys (Utilities|Map|Keys (Variables|Default|GetUnitTeams)))
    (for _array_element _keys
      (bind _output_get (LocalVariables|SetTeamIndex _array_element))
      (bind _result (Utilities|Set|ToArray (Utilities|Struct|BreakSTR_UnitSet (.Value (Utilities|Map|Find (Variables|Default|GetUnitTeams) _output_get)))))
      (bind _array_element_2 (Utilities|Array|ForEachLoopwithBreak _result :!label _label)
        (:LoopBody
          (if (Default|IsAlive _array_element_2)
            (Utilities|Array|Add (LocalVariables|GetTeamsAlive) (LocalVariables|GetTeamIndex))
            (goto _label Break)))
        (:Completed
          (if (== (Utilities|Array|Length _teamsalive) 1)
            (CallFunction|FinishCombat (Utilities|Array|Get(acopy) _teamsalive))))))
    (else
      (Default|DebugRespawnAfterDelay Unit))))

(fn FinishCombat
  (params (WinningTeamIndex :type Integer))
  (Variables|Default|SetIsFinishingCombat true)
  (Default|CallOnCombatFinishing WinningTeamIndex))