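; Player grid action that adds a tile to the grid at a given index.
; Execute Action runs only when the index is not already valid on the BPGrid held by BPPlayerActions.
; It traces for ground at the index's location to place the tile, takes rotation and scale from the grid, and registers it with a fixed tile type through AddGridTile.
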(fn ConstructionScript
  (|CallParentFunction))

(fn ExecuteAction
  (params (Index :type Int%20Point%20Structure))
  (bind _bp_playeractions (Variables|Default|GetBP_PlayerActions))
  (bind _bp_grid (Variables|/Game/2-Blueprints/Core/Player/BP_PlayerActions.BP_PlayerActions_C|GetBP_Grid _bp_playeractions))
  (if (not (Default|IsIndexValid (Variables|/Game/2-Blueprints/Core/Player/BP_PlayerActions.BP_PlayerActions_C|GetBP_Grid (Variables|Default|GetBP_PlayerActions)) Index))
    (bind _out_location (Default|TraceforGround (Variables|/Game/2-Blueprints/Core/Player/BP_PlayerActions.BP_PlayerActions_C|GetBP_Grid (Variables|Default|GetBP_PlayerActions)) (Default|GetTileLocationfromGridIndex _bp_grid Index)))
    (Default|AddGridTile (Variables|/Game/2-Blueprints/Core/Player/BP_PlayerActions.BP_PlayerActions_C|GetBP_Grid (Variables|Default|GetBP_PlayerActions)) (Utilities|Struct|MakeSTR_TileData Index "NewEnumerator1" (Math|Transform|MakeTransform _out_location (Default|GetTileRotationfromGridIndex _bp_grid Index) (Default|GetTileScalefromGridIndex _bp_grid Index)) "NewEnumerator0" 0))))