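; BP_SpellAnimation is a short-lived actor that plays the visual of a spell hitting its attacked grid tiles.
; On BeginPlay it spawns a BP_AnimatedShape per attacked tile, animating the grid's shape mesh from the origin tile to that tile with randomized red brightness and play rate.
; Each finished shape broadcasts a tile-hit event; once none remain, the actor broadcasts completion and destroys itself.
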(event Custom|Event_PlaySpellAnimation
  (bind _bp_grid (Variables|Default|GetBP_Grid))
  (bind _originindex (Variables|Default|GetOriginIndex))
  (bind _data (Default|GetCurrentShapeData _bp_grid))
  (bind _transform (CallFunction|GetTileTransform _originindex))
  (bind (_mesh _flatmaterial) (Utilities|Struct|BreakSTR_GridShapesData _data))
  (for _array_element (Variables|Default|GetAttackedIndexes)
    (bind _returnvalue (Game|SpawnActorfromClass "/Game/2-Blueprints/Core/Combat/Spells/SpellAnimation/Components/BP_AnimatedShape.BP_AnimatedShape_C" (Math|Transform|MakeTransform "0, 0, 0" "0, 0, 0" "1.000000,1.000000,1.000000") "Undefined" "MultiplyWithRoot" 0 _mesh _flatmaterial (* "(R=0.921875,G=0.053612,B=0.000000,A=1.000000)" (Math|Random|RandomFloatinRange 0.5 1.5)) (Math|Transform|MakeTransform (.location _transform) (.rotation _transform) "0.010000,0.010000,0.010000") (CallFunction|GetTileTransform _array_element) (Math|Random|RandomFloatinRange 0.5 1.5) _array_element 0))
    (EventDispatchers|BindEventtoOnShapeAnimationCompleted _returnvalue (delegate Custom|OnShapeAnimationCompleted))))

(event Custom|OnShapeAnimationCompleted
  (params (AnimatedShape :type BP%20Animated%20Shape%20Object%20Reference))
  (bind _attackedindexes (Variables|Default|GetAttackedIndexes))
  (bind _index (Variables|/Game/2-Blueprints/Core/Combat/Spells/SpellAnimation/Components/BP_AnimatedShape.BP_AnimatedShape_C|GetIndex AnimatedShape))
  (Default|CallOnSpellAnimationHitTile self _index)
  (Utilities|Array|RemoveItem _attackedindexes _index)
  (if (== (Utilities|Array|Length _attackedindexes) 0)
    (CallFunction|EventCompleteSpellAnimation)))

(event Custom|Event_CompleteSpellAnimation
  (Default|CallOnSpellAnimationCompleted self)
  (Actor|DestroyActor))

(event EventBeginPlay
  (CallFunction|EventPlaySpellAnimation))

(fn ConstructionScript)

(fn GetTileTransform
  (params (Index :type Int%20Point%20Structure%20%28by%20ref%29))
  (return (Utilities|Struct|BreakSTR_TileData (.Value (Utilities|Map|Find (Variables|/Game/2-Blueprints/Core/Grid/BP_Grid.BP_Grid_C|GetGridTiles (Variables|Default|GetBP_Grid)) Index)))))