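; BP_GridModifier is a grid marker actor with a shape and a tile type, such as obstacle, higher movement cost or flying-only.
; Its construction script applies the shape's mesh and flat material, then tints it filled with a color per type.
; It sets overlap and block responses on two custom trace channels and hides itself in game.
; The event graph holds no logic.
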(event EventBeginPlay)

(event Collision|EventActorBeginOverlap
  (params (OtherActor :type Actor%20Object%20Reference)))

(event EventTick
  (params (DeltaSeconds :type Float%20%28single-precision%29)))

(fn ConstructionScript
  (bind _staticmesh (Variables|Default|GetStaticMesh))
  (bind _shape (Variables|Default|GetShape))
  (bind _staticmesh_2 (Variables|Default|GetStaticMesh))
  (bind _data (CallFunction|GetShapeData _shape))
  (Components|StaticMesh|SetStaticMesh _staticmesh (.mesh _data))
  (Rendering|Material|SetMaterial _staticmesh 0 (.flatmaterial _data))
  (Rendering|Material|SetVectorParameterValueonMaterials (Variables|Default|GetStaticMesh) "Color" (Math|Conversions|ToVector(LinearColor) (Utilities|Select :Index (Variables|Default|GetType) :NewEnumerator0 "" :NewEnumerator1 "(R=1.000000,G=1.000000,B=1.000000,A=1.000000)" :NewEnumerator2 "(R=1.000000,G=0.047444,B=0.000000,A=1.000000)" :NewEnumerator4 "(R=0.578125,G=0.524319,B=0.248884,A=1.000000)" :NewEnumerator5 "(R=0.165620,G=0.744792,B=0.140993,A=1.000000)" :NewEnumerator6 "(R=0.255845,G=0.530546,B=0.546875,A=1.000000)")))
  (Rendering|Material|SetScalarParameterValueonMaterials (Variables|Default|GetStaticMesh) "IsFilled" 1.0)
  (Collision|SetCollisionResponsetoChannel _staticmesh_2 "ECC_GameTraceChannel1" "ECR_Overlap")
  (Collision|SetCollisionResponsetoChannel _staticmesh_2 "ECC_GameTraceChannel4" "ECR_Block")
  (Rendering|SetActorHiddenInGame true))