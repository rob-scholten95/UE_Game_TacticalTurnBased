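; BP_GridVisual renders the tiles of a BP_Grid in a flat view and a tactical view.
; It feeds tile updates to two child BP_GridMeshInst actors, keeping flat tiles walkable-only and offset from the ground.
; Tactical tiles are colored by type and stretched in Z relative to the lowest tile.
; Tactical mode hides "NotTactical"-tagged actors and lazily rebuilds its instances when flagged stale.
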(event EventBeginPlay
  (Actor|Tick|SetActorTickEnabled false))

(event Collision|EventActorBeginOverlap
  (params (OtherActor :type Actor%20Object%20Reference)))

(event EventTick
  (params (DeltaSeconds :type Float%20%28single-precision%29)))

(fn ConstructionScript)

(fn InitializeGridVisual
  (params (BP_Grid :type BP%20Grid%20Object%20Reference))
  ;[1 1 1] Setting the current BP_Grid Object
  (Variables|Components|SetBP%20Grid BP_Grid)
  ;[1 1 1] Getting and Storing the BP_GridMeshInst object
  (Variables|Default|SetBP%20Grid%20Mesh%20Inst (.AsBP%20Grid%20Mesh%20Inst (Utilities|Casting|CastToBP_GridMeshInst (Variables|/Script/Engine.ChildActorComponent|GetChildActor (Variables|Default|GetChildActor_GridMeshInst)))))
  (Variables|Default|SetAs%20BP%20Grid%20Mesh%20Inst_Tactical (.AsBP%20Grid%20Mesh%20Inst (Utilities|Casting|CastToBP_GridMeshInst (Variables|/Script/Engine.ChildActorComponent|GetChildActor (Variables|Default|GetChildActor_GridMeshInst_Tactical)))))
  (Default|InitializeGridMeshInstances (Variables|Default|GetBP%20Grid%20Mesh%20Inst) (.flatmesh (Default|GetCurrentShapeData (Variables|Components|GetBP%20Grid))) (.flatmaterial (Default|GetCurrentShapeData (Variables|Components|GetBP%20Grid))) false "QueryOnly")
  (Default|InitializeGridMeshInstances (Variables|Default|GetAs%20BP%20Grid%20Mesh%20Inst_Tactical) (.mesh (Default|GetCurrentShapeData (Variables|Components|GetBP%20Grid))) (.meshinstance (Default|GetCurrentShapeData (Variables|Components|GetBP%20Grid))) true "QueryOnly")
  (Transformation|SetActorLocation "0, 0, 0" false false)
  (CallFunction|SetOffsetfromGround (Variables|Default|GetOffsetFromGround))
  (CallFunction|SetGridLowestZ 9999999.0)
  (CallFunction|SetIsTactical (Variables|Default|GetIsTactical)))

(fn SetOffsetfromGround
  (params (Offset :type Float%20%28double-precision%29))
  (Variables|Default|SetOffsetFromGround Offset)
  (Transformation|SetRelativeLocation (Variables|Default|GetChildActor_GridMeshInst) (Math|Vector|MakeVector 0.0 0.0 (Variables|Default|GetOffsetFromGround)) false false))

(fn DestroyGridVisual
  (bind _as_bp_grid_mesh_inst_tactical (Variables|Default|GetAs%20BP%20Grid%20Mesh%20Inst_Tactical))
  (bind _bp_grid_mesh_inst (Variables|Default|GetBP%20Grid%20Mesh%20Inst))
  (Utilities|FlowControl|Sequence
    (:then_0
      ;[1 1 1] Checking whether the grid instance is valid
      (Utilities|IsValid _bp_grid_mesh_inst
        (:Is%20Valid
          ;[1 1 1] Clear all the instances in Grid Mesh inst
          (Default|ClearInstances _bp_grid_mesh_inst))))
    (:then_1
      ;[1 1 1] Checking whether the grid instance is valid
      (Utilities|IsValid _as_bp_grid_mesh_inst_tactical
        (:Is%20Valid
          ;[1 1 1] Clear all the instances in Grid Mesh inst
          (Default|ClearInstances _as_bp_grid_mesh_inst_tactical))))
    (:then_2
      (CallFunction|SetGridLowestZ 9999999.0))))

(fn UpdateTileVisual
  (params (Data :type STR%20Tile%20Data%20Structure))
  (Utilities|FlowControl|Sequence
    (:then_0
      (Default|RemoveInstance (Variables|Default|GetBP%20Grid%20Mesh%20Inst) (.index Data))
      (if (CallFunction|IsTileWalkable (.tiletype Data))
        (Default|AddInstance (Variables|Default|GetBP%20Grid%20Mesh%20Inst) (.index Data) (.transform Data) (.tilestate Data) (.tiletype Data))))
    (:then_1
      (CallFunction|UpdateTileVisualTactical Data))))

(fn UpdateTileVisualTactical
  (params (Data :type STR%20Tile%20Data%20Structure))
  (bind _bp_grid (Variables|Components|GetBP%20Grid))
  (bind (_location _rotation _scale) (Math|Transform|BreakTransform (.transform Data)))
  (bind _location_2 (Math|Transform|BreakTransform (.transform Data)))
  (bind _data (Default|GetCurrentShapeData _bp_grid))
  (bind _meshsize (Utilities|Struct|BreakSTR_GridShapesData _data))
  (bind (_x _y) (Class|KismetMathLibrary|BreakVector3f _scale))
  (bind _z (Class|KismetMathLibrary|BreakVector3f _location_2))
  (bind _z_2 (Class|KismetMathLibrary|BreakVector3f _meshsize))
  (Utilities|FlowControl|Sequence
    (:then_0
      (if (< _z (Variables|Default|GetGridLowestZ))
        (CallFunction|SetGridLowestZ _z)))
    (:then_1
      (if (Variables|Default|GetIsTactical)
        (Default|RemoveInstance (Variables|Default|GetAs%20BP%20Grid%20Mesh%20Inst_Tactical) (.index Data))
        (if (Utilities|Enum|NotEqual(Enum) (.tiletype Data) "NewEnumerator0")
          (Default|AddInstance (Variables|Default|GetAs%20BP%20Grid%20Mesh%20Inst_Tactical) (.index Data) (Math|Transform|MakeTransform _location _rotation (Math|Vector|MakeVector _x _y (/ (+ (- (.Z (Class|KismetMathLibrary|BreakVector3f (.Location (Math|Transform|BreakTransform (.transform Data))))) (Variables|Default|GetGridLowestZ)) _z_2) _z_2))) (.tilestate Data) (.tiletype Data)))
        (else
          (Variables|Components|SetNeedToReGenerateTacticalOnNextEnable true))))))

(fn SetGridLowestZ
  (params (GridLowestZ :type Float%20%28double-precision%29))
  (Variables|Default|SetGridLowestZ GridLowestZ)
  (Variables|Components|SetNeedToReGenerateTacticalOnNextEnable true))

(fn SetIsTactical
  (params (IsTactical :type Boolean))
  (Variables|Default|SetIsTactical IsTactical)
  (Development|SetHiddeninGame (Variables|Default|GetChildActor_GridMeshInst_Tactical) (not (Variables|Default|GetIsTactical)) false)
  (bind _outactors (Actor|GetAllActorswithTag "NotTactical"))
  (for _array_element _outactors
    (Rendering|SetActorHiddenInGame _array_element (Variables|Default|GetIsTactical))
    (if (and (Variables|Default|GetIsTactical) (Variables|Components|GetNeedToReGenerateTacticalOnNextEnable))
      (Variables|Components|SetNeedToReGenerateTacticalOnNextEnable false)
      (bind _values (Utilities|Map|Values (Variables|/Game/2-Blueprints/Core/Grid/BP_Grid.BP_Grid_C|GetGridTiles (Variables|Components|GetBP%20Grid))))
      (for _array_element_2 _values
        (CallFunction|UpdateTileVisualTactical _array_element_2)))))