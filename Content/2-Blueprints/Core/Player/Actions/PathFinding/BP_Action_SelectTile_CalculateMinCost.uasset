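; Player grid action that fills pathfinding data with each tile's minimum cost to the selected tile, without running a path search.
; On execute it runs the parent action, then clears the grid pathfinding component's generated data.
; If the selected tile index is valid, it loops over every grid tile, computes that cost with the diagonals option, and registers the tile through DiscoverTile.
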(event EventBeginPlay
  (|CallParentFunction) ; This node is disabled and will not be called.\nDrag off pins to build functionality.
)

(event Collision|EventActorBeginOverlap
  (params (OtherActor :type Actor%20Object%20Reference))
  (|CallParentFunction OtherActor) ; This node is disabled and will not be called.\nDrag off pins to build functionality.
)

(event EventTick
  (params (DeltaSeconds :type Float%20%28single-precision%29))
  (|CallParentFunction DeltaSeconds) ; This node is disabled and will not be called.\nDrag off pins to build functionality.
)

(fn ConstructionScript
  (|CallParentFunction))

(fn ExecuteAction
  (params (Index :type Int%20Point%20Structure))
  (bind _bp_playeractions (Variables|Default|GetBP_PlayerActions))
  (bind _bp_playeractions_2 (Variables|Default|GetBP_PlayerActions))
  (bind _bp_grid (Variables|/Game/2-Blueprints/Core/Player/BP_PlayerActions.BP_PlayerActions_C|GetBP_Grid _bp_playeractions))
  ;[1 1 1] Comment
  (|CallParentFunction Index)
  ;[1 1 1] Comment
  (Default|ClearGeneratedData (Variables|/Game/2-Blueprints/Core/Grid/BP_Grid.BP_Grid_C|GetBP_GridPathFinding (Variables|/Game/2-Blueprints/Core/Player/BP_PlayerActions.BP_PlayerActions_C|GetBP_Grid (Variables|Default|GetBP_PlayerActions))))
  ;[1 1 1] Comment
  (if (Default|IsIndexValid (Variables|/Game/2-Blueprints/Core/Player/BP_PlayerActions.BP_PlayerActions_C|GetBP_Grid _bp_playeractions_2) (Variables|/Game/2-Blueprints/Core/Player/BP_PlayerActions.BP_PlayerActions_C|GetSelectedTileIndex _bp_playeractions_2))
    ;[1 1 1] Comment
    (bind _keys (Utilities|Map|Keys (Variables|/Game/2-Blueprints/Core/Grid/BP_Grid.BP_Grid_C|GetGridTiles _bp_grid)))
    (for _array_element _keys
      (Default|DiscoverTile (Variables|/Game/2-Blueprints/Core/Grid/BP_Grid.BP_Grid_C|GetBP_GridPathFinding (Variables|/Game/2-Blueprints/Core/Player/BP_PlayerActions.BP_PlayerActions_C|GetBP_Grid (Variables|Default|GetBP_PlayerActions))) (Utilities|Struct|MakeSTR_PathFindingData _array_element 1 999999 (Default|GetMinimumCostBetweenTwoTiles (Variables|/Game/2-Blueprints/Core/Grid/BP_Grid.BP_Grid_C|GetBP_GridPathFinding _bp_grid) _array_element (Variables|/Game/2-Blueprints/Core/Player/BP_PlayerActions.BP_PlayerActions_C|GetSelectedTileIndex _bp_playeractions) (Variables|Default|GetIncludeDiagonals)) "(X=-999,Y=-999)")))))