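; Spell animation actor for Sword Throw that flies from an origin tile to a target tile.
; On play it faces the target using the tile indices, then a Timeline lerps its location between the two tiles.
; The same Timeline drives the Anim component's sideways offset, yaw spin and scale.
; A DoOnce fires the tile-hit callback once playback passes a fixed time, and the Timeline's end completes the animation.
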(event EventBeginPlay
  (|CallParentFunction) ; This node is disabled and will not be called.\nDrag off pins to build functionality.
)

(event Collision|EventActorBeginOverlap
  (params (OtherActor :type Actor%20Object%20Reference)))

(event EventTick
  (params (DeltaSeconds :type Float%20%28single-precision%29)))

(event EventEventPlaySpellAnimation
  (Transformation|SetActorLocationAndRotation (.location (CallFunction|GetTileTransform (Variables|Default|GetOriginIndex))) (Math|Rotator|FindLookatRotation (Math|Conversions|ToVector(Vector2D) (Math|Conversions|ToVector2D(IntPoint) (Variables|Default|GetOriginIndex))) (Math|Conversions|ToVector(Vector2D) (Math|Conversions|ToVector2D(IntPoint) (Variables|Default|GetTargetIndex)))))
  (bind (_direction _actorlocationalpha _rotationz _scale _locationy) (Timeline|Timeline PlayFromStart)
    (:Update
      (Utilities|FlowControl|Sequence
        (:then_0
          (Transformation|SetActorLocation (Math|Vector|Lerp(Vector) (.location (CallFunction|GetTileTransform (Variables|Default|GetOriginIndex))) (.location (CallFunction|GetTileTransform (Variables|Default|GetTargetIndex))) _actorlocationalpha) false false))
        (:then_1
          (Transformation|SetRelativeTransform (Variables|Default|GetAnim) (Math|Transform|MakeTransform (Math|Vector|MakeVector 0.0 _locationy 0.0) (Math|Rotator|MakeRotator 0.0 0.0 _rotationz) (Math|Conversions|ToVector(Float) _scale)) false false)
          (if (>= (Components|Timeline|GetPlaybackPosition (Variables|Default|GetTimeline)) 0.28)
            (Utilities|FlowControl|DoOnce false
              (:Completed
                (Default|CallOnSpellAnimationHitTile self (Variables|Default|GetTargetIndex))))))))
    (:Finished
      (CallFunction|EventCompleteSpellAnimation))))

(fn ConstructionScript
  (|CallParentFunction))