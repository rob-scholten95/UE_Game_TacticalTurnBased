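; Grid-based tactics unit that loads mesh, anim class and stats from its unit type, with team-colored tile marker, health bar and selection highlight.
; A timeline walks it tile by tile along paths, adding a jump across height changes.
; Stat setters clamp HP, AP and MP and broadcast changes.
; Spell hits change HP immediately but defer health bar, numbers and hit/death animations until the spell animation reaches the tile.
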(event Custom|Follow%20Path
  (params (Path :type Array%20of%20Int%20Point%20Structures))
  ;[1 1 1] Comment
  (if (> (Utilities|Array|Length Path) 0)
    (Variables|Default|SetCurrentPathToFollow Path)
    (Default|CallOnUnitStartWalking self)
    (CallFunction|ContinuetoFollowPath)))

(event Custom|ContinueToFollowPath
  (bind _bp_grid (Variables|Default|GetBP_Grid))
  (bind _currentpathtofollow (Variables|Default|GetCurrentPathToFollow))
  (bind _timeline_unitmovement (Variables|Default|GetTimeline_UnitMovement))
  (bind _output (Utilities|Array|Get(acopy) _currentpathtofollow))
  (bind _gridtiles (Variables|/Game/2-Blueprints/Core/Grid/BP_Grid.BP_Grid_C|GetGridTiles _bp_grid))
  (bind _value (Utilities|Map|Find _gridtiles _output))
  (bind _transform (Utilities|Struct|BreakSTR_TileData _value))
  ;[1 1 1] Comment
  (if (> (Utilities|Array|Length (Variables|Default|GetCurrentPathToFollow)) 0)
    (Animations|SetUnitAnimationState "NewEnumerator1")
    (Variables|Default|SetPreviousTransform (Transformation|GetActorTransform))
    (Variables|Default|SetNextTransform (Math|Transform|MakeTransform (.location _transform) (Math|Rotator|MakeRotator 0.0 0.0 (.yaw (Math|Rotator|FindLookatRotation (.location (Variables|Default|GetPreviousTransform)) (.location _transform)))) "1.000000,1.000000,1.000000"))
    (Components|Timeline|SetPlayRate _timeline_unitmovement (/ (Components|Timeline|GetTimelineLength _timeline_unitmovement) (Variables|Default|GetMoveDurationPerTile)))
    (bind (_direction _locationalpha _rotationalpha _jump) (Timeline|Timeline_UnitMovement PlayFromStart)
      (:Update
        (Transformation|SetActorLocationAndRotation (+ (Math|Vector|Lerp(Vector) (.location (Variables|Default|GetPreviousTransform)) (.location (Variables|Default|GetNextTransform)) _locationalpha) (Math|Vector|MakeVector 0.0 0.0 (Math|Float|SelectFloat 0.0 _jump (Math|Float|NearlyEqual(Float) (.z (.location (Variables|Default|GetPreviousTransform))) (.z (.location (Variables|Default|GetNextTransform))) 5.0)))) (Math|Rotator|Lerp(Rotator) (.rotation (Variables|Default|GetPreviousTransform)) (.rotation (Variables|Default|GetNextTransform)) _rotationalpha true)))
      (:Finished
        (Default|CallOnUnitReachedNewTile self (Utilities|Array|Get(acopy) (Variables|Default|GetCurrentPathToFollow)))
        (Utilities|Array|RemoveIndex (Variables|Default|GetCurrentPathToFollow))
        (CallFunction|ContinuetoFollowPath)))
    (else
      (Animations|SetUnitAnimationState "NewEnumerator0")
      (Default|CallOnUnitFinishedWalking self))))

(event Custom|Debug_RespawnAfterDelay
  ;[1 1 1] Comment
  (Utilities|FlowControl|Delay 2.0)
  (HP|SetCurrentHP (.HP_Max (Utilities|Struct|BreakSTR_UnitData_Stats (Utilities|Struct|BreakSTR_UnitData (Variables|Default|GetUnitData)))))
  (Animations|SetUnitAnimationState "NewEnumerator5")
  (Default|EventUpdateHPBar (Variables|Default|GetUW_HealthBar)))

(event Custom|Event_HideUnitAfterSeconds
  ;[1 1 1] Comment
  (Utilities|FlowControl|Delay 2.0)
  (if (not (CallFunction|IsAlive))
    (Transformation|SetActorLocation "-99999.000000,-99999.000000,-99999.000000" false false)))

(event EventBeginPlay
  ;[1 1 1] Comment
  (Animations|SetUnitAnimationState "NewEnumerator0")
  (bind _output_get (Variables|Default|SetUW_HealthBar (.AsUW%20Health%20Bar (Utilities|Casting|CastToUW_HealthBar (UserInterface|GetUserWidgetObject (Variables|Default|GetWidget_Healthbar))))))
  (Default|EventSetUnit _output_get self))

(fn ConstructionScript
  (bind _unit_data (CallFunction|GetDefaultDatafromUnitType (Variables|Default|GetUnitType)))
  (UnitData|SetUnitData _unit_data)
  (Grid|UpdateVisualUnit))

(fn UpdateVisualUnit
  (Rendering|Material|SetVectorParameterValueonMaterials (Variables|Default|GetSkeletalMesh) "ColorMultiply" (Math|Conversions|ToVector(LinearColor) (* (* (select (Variables|Default|GetIsSelected) "(R=0.103953,G=0.583333,B=0.107672,A=1.000000)" "(R=1.000000,G=1.000000,B=1.000000,A=1.000000)") (select (Variables|Default|GetIsHovered) 2.5 1.0)) (select (Variables|Default|GetIsSelected) 3.0 1.0)))))

(fn SetIsHovered
  (params (IsHovered :type Boolean))
  (Variables|Default|SetIsHovered IsHovered)
  (Grid|UpdateVisualUnit)
  (Default|CallOnUnitHoveredChanged self))

(fn SetIsSelected
  (params (IsSelected :type Boolean))
  (Variables|Default|SetIsSelected IsSelected)
  (Grid|UpdateVisualUnit)
  (Default|CallOnUnitSelectedChanged self))

(fn SetUnitData
  (params (Data :type STR%20Unit%20Data%20Structure%20%28by%20ref%29))
  (bind _skeletalmesh (Variables|Default|GetSkeletalMesh))
  (bind _uw_healthbar (Variables|Default|GetUW_HealthBar))
  (bind _output_get (Variables|Default|SetUnitData Data))
  (Components|SkeletalMesh|SetSkeletalMeshAsset _skeletalmesh (.mesh (.Assets (Utilities|Struct|BreakSTR_UnitData _output_get))))
  (Class|SkeletalMeshComponent|SetAnimClass _skeletalmesh (.animbp (.Assets (Utilities|Struct|BreakSTR_UnitData _output_get))))
  (Default|CallOnUnitStatsChanged self)
  (Utilities|IsValid _uw_healthbar
    (:Is%20Valid
      (Default|EventUpdateHPBar _uw_healthbar))))

(fn SetUnitAnimationState
  (params (State :type EN_UnitAnimationState%20Enum :default "NewEnumerator0"))
  (Class|BPIUnitAnimation|SetUnitAnimationState(Message) (Components|SkeletalMesh|GetAnimInstance (Variables|Default|GetSkeletalMesh)) State))

(fn SetGrid
  (params (BP_Grid :type BP%20Grid%20Object%20Reference))
  (bind _collision_los (Variables|Default|GetCollision_LOS))
  (bind _mesh_teamindex (Variables|Default|GetMesh_TeamIndex))
  (Variables|Default|SetBP_Grid BP_Grid)
  ;[1 1 1] Comment
  (Components|StaticMesh|SetStaticMesh _collision_los (.Mesh (Utilities|Struct|BreakSTR_GridShapesData (Default|GetCurrentShapeData (Variables|Default|GetBP_Grid)))))
  (Transformation|SetAbsolute _collision_los false true true)
  (Transformation|SetWorldScale3D (Variables|Default|GetCollision_LOS) (Math|Vector|MakeVector (.x (/ (Variables|/Game/2-Blueprints/Core/Grid/BP_Grid.BP_Grid_C|GetTile%20Size (Variables|Default|GetBP_Grid)) (.MeshSize (Utilities|Struct|BreakSTR_GridShapesData (Default|GetCurrentShapeData (Variables|Default|GetBP_Grid)))))) (.y (/ (Variables|/Game/2-Blueprints/Core/Grid/BP_Grid.BP_Grid_C|GetTile%20Size (Variables|Default|GetBP_Grid)) (.MeshSize (Utilities|Struct|BreakSTR_GridShapesData (Default|GetCurrentShapeData (Variables|Default|GetBP_Grid)))))) (.z (Transformation|GetWorldScale (Variables|Default|GetCollision_LOS)))))
  (Transformation|SetWorldRotation (Variables|Default|GetCollision_LOS) (Default|GetTileRotationfromGridIndex (Variables|Default|GetBP_Grid) (Variables|Default|GetIndex)) false false)
  ;[1 1 1] Comment
  (Components|StaticMesh|SetStaticMesh _mesh_teamindex (.FlatMesh (Utilities|Struct|BreakSTR_GridShapesData (Default|GetCurrentShapeData (Variables|Default|GetBP_Grid)))))
  (Rendering|Material|SetMaterial _mesh_teamindex 0 (.FlatMaterial (Utilities|Struct|BreakSTR_GridShapesData (Default|GetCurrentShapeData (Variables|Default|GetBP_Grid)))))
  (Rendering|Material|SetScalarParameterValueonMaterials _mesh_teamindex "IsFilled" 1.0)
  (Transformation|SetAbsolute _mesh_teamindex false true true)
  (Transformation|SetWorldScale3D _mesh_teamindex (/ (Variables|/Game/2-Blueprints/Core/Grid/BP_Grid.BP_Grid_C|GetTile%20Size (Variables|Default|GetBP_Grid)) (.MeshSize (Utilities|Struct|BreakSTR_GridShapesData (Default|GetCurrentShapeData (Variables|Default|GetBP_Grid))))))
  (Transformation|SetWorldRotation _mesh_teamindex (Default|GetTileRotationfromGridIndex (Variables|Default|GetBP_Grid) (Variables|Default|GetIndex)) false false)
  (Transformation|SetRelativeLocation _mesh_teamindex (Math|Vector|MakeVector 0.0 0.0 (+ (Variables|/Game/2-Blueprints/Core/Grid/BP_GridVisual.BP_GridVisual_C|GetOffsetFromGround (Variables|/Game/2-Blueprints/Core/Grid/BP_Grid.BP_Grid_C|GetBP_Grid%20Visual (Variables|Default|GetBP_Grid))) 5.0)) false false))

(fn SetGridIndex
  (params (Index :type Int%20Point%20Structure))
  (Variables|Default|SetIndex Index)
  (Transformation|SetWorldRotation (Variables|Default|GetCollision_LOS) (Default|GetTileRotationfromGridIndex (Variables|Default|GetBP_Grid) (Variables|Default|GetIndex)) false false))

(fn UnitCastSpell
  (params (Target%20Index :type Int%20Point%20Structure) (Spell%20Data :type STR%20Spell%20Data%20Structure))
  (bind _self self)
  (bind _bp_grid (Variables|Default|GetBP_Grid))
  (bind _returnvalue (Transformation|GetActorLocation _self))
  (bind _gridtiles (Variables|/Game/2-Blueprints/Core/Grid/BP_Grid.BP_Grid_C|GetGridTiles _bp_grid))
  (bind _value (Utilities|Map|Find _gridtiles Target%20Index))
  (bind _transform (Utilities|Struct|BreakSTR_TileData _value))
  (bind _location (Math|Transform|BreakTransform _transform))
  (bind (_x _y) (Class|KismetMathLibrary|BreakVector3f _location))
  (Transformation|SetActorRotation (Math|Rotator|FindLookatRotation (Math|Vector|MakeVector (.x _returnvalue) (.y _returnvalue) 0.0) (Math|Vector|MakeVector _x _y 0.0)))
  (Animations|SetUnitAnimationState "NewEnumerator2")
  (AP|ModifyCurrentAP (Utilities|Struct|BreakSTR_SpellData_Requirements (Utilities|Struct|BreakSTR_SpellData Spell%20Data)) true))

(fn SetCurrentHP
  (params (HP :type Integer))
  (bind _structout (Utilities|Struct|SetmembersinSTR_UnitData_Stats (Utilities|Struct|BreakSTR_UnitData (Variables|Default|GetUnitData)) (Math|Integer|Clamp(Integer) HP 0 (.HP_Max (Utilities|Struct|BreakSTR_UnitData_Stats (Utilities|Struct|BreakSTR_UnitData (Variables|Default|GetUnitData)))))))
  (Utilities|Struct|SetmembersinSTR_UnitData (Variables|Default|GetUnitData) _structout)
  (Default|CallOnUnitStatsChanged self))

(fn ModifyCurrentHP
  (params (Modifier :type Integer))
  (HP|SetCurrentHP (+ Modifier (.HP_Current (Utilities|Struct|BreakSTR_UnitData_Stats (Utilities|Struct|BreakSTR_UnitData (Variables|Default|GetUnitData)))))))

(fn UnitHitbySpell
  (params (SpellImpactReal :type STR%20Spell%20Data%20Impact%20Real%20Structure) (SpellAnimation :type BP%20Spell%20Animation%20Object%20Reference))
  (bind _modifier_hp (Utilities|Struct|BreakSTR_SpellData_Impact_Real SpellImpactReal))
  (Utilities|Map|Add (Variables|Default|GetIncomingSpells) SpellAnimation SpellImpactReal)
  (EventDispatchers|BindEventtoOnSpellAnimationHitTile SpellAnimation (EventDispatchers|CreateEvent :!event OnSpellAnimationHitTile))
  (if (!= _modifier_hp 0)
    (HP|ModifyCurrentHP _modifier_hp)))

(fn OnSpellAnimationHitTile
  (params (SpellAnimation :type BP%20Spell%20Animation%20Object%20Reference) (Tile%20Index :type Int%20Point%20Structure))
  (bind _incomingspells (Variables|Default|GetIncomingSpells))
  (bind (_value _returnvalue) (Utilities|Map|Find _incomingspells SpellAnimation))
  (if (Class|KismetMathLibrary|EqualIntPointIntPoint (Variables|Default|GetIndex) Tile%20Index)
    (if _returnvalue :!label _label
      (LocalVariables|SetSpellImpactReal _value)
      (Utilities|Map|Remove (Variables|Default|GetIncomingSpells) SpellAnimation)
      (Default|EventUpdateHPBar (Variables|Default|GetUW_HealthBar))
      (if (!= (Utilities|Struct|BreakSTR_SpellData_Impact_Real (LocalVariables|GetSpellImpactReal)) 0)
        (Game|SpawnActorfromClass "/Game/2-Blueprints/Core/Units/Widget/BP_AnimatedNumber.BP_AnimatedNumber_C" (Math|Transform|MakeTransform (Transformation|GetActorLocation) "0, 0, 0" "1.000000,1.000000,1.000000") "Undefined" "MultiplyWithRoot" 0 (Utilities|Struct|BreakSTR_SpellData_Impact_Real (LocalVariables|GetSpellImpactReal)) "NewEnumerator0" 0)
        (if (< (Utilities|Struct|BreakSTR_SpellData_Impact_Real (LocalVariables|GetSpellImpactReal)) 0)
          (if (not (CallFunction|IsAlive))
            (Animations|SetUnitAnimationState "NewEnumerator4")
            (else
              (Animations|SetUnitAnimationState "NewEnumerator3"))))))
    (elif (Class|KismetMathLibrary|EqualIntPointIntPoint (Variables|Default|GetIndexToRememberForSpellImpact) Tile%20Index)
      (Variables|Default|SetIndexToRememberForSpellImpact (Utilities|Struct|MakeIntPoint -999 -999))
      (goto _label))))

(fn SetTeamIndex
  (params (Index :type Integer))
  (Variables|Default|SetTeamIndex Index)
  ;[1 1 1] Comment
  (Class|ProgressBar|SetFillColorandOpacity (Variables|/Game/2-Blueprints/Core/Units/Widget/UW_HealthBar.UW_HealthBar_C|GetProgressBar_HP (Variables|Default|GetUW_HealthBar)) (CallFunction|GetTeamColor (Variables|Default|GetTeamIndex)))
  (Rendering|Material|SetVectorParameterValueonMaterials (Variables|Default|GetMesh_TeamIndex) "Color" (Math|Conversions|ToVector(LinearColor) (CallFunction|GetTeamColor (Variables|Default|GetTeamIndex)))))

(fn CombatStarted
  (MP|ResetMP)
  (AP|ResetAP))

(fn TurnStarted)

(fn TurnEnded
  (MP|ResetMP)
  (AP|ResetAP))

(fn CombatEnded
  (MP|ResetMP)
  (AP|ResetAP))

(fn SetCurrentMP
  (params (MP :type Integer) (Show%20Number :type Boolean))
  (bind _unitdata (Variables|Default|GetUnitData))
  (bind _stats (Utilities|Struct|BreakSTR_UnitData _unitdata))
  (bind (_mp_current _mp_max) (Utilities|Struct|BreakSTR_UnitData_Stats _stats))
  (LocalVariables|SetDifference (- MP _mp_current))
  (bind _structout (Utilities|Struct|SetmembersinSTR_UnitData_Stats (Utilities|Struct|BreakSTR_UnitData (Variables|Default|GetUnitData)) (Math|Integer|Clamp(Integer) MP 0 _mp_max)))
  (Utilities|Struct|SetmembersinSTR_UnitData (Variables|Default|GetUnitData) _structout)
  (Default|CallOnUnitStatsChanged self)
  (if (and Show%20Number (!= (LocalVariables|GetDifference) 0))
    (Game|SpawnActorfromClass "/Game/2-Blueprints/Core/Units/Widget/BP_AnimatedNumber.BP_AnimatedNumber_C" (Math|Transform|MakeTransform (Transformation|GetActorLocation) "0, 0, 0" "1.000000,1.000000,1.000000") "Undefined" "MultiplyWithRoot" 0 (LocalVariables|GetDifference) "NewEnumerator1" 0)))

(fn ModifyCurrentMP
  (params (Modifier :type Integer) (Show%20Number :type Boolean))
  (MP|SetCurrentMP (+ Modifier (.MP_Current (Utilities|Struct|BreakSTR_UnitData_Stats (Utilities|Struct|BreakSTR_UnitData (Variables|Default|GetUnitData))))) Show%20Number))

(fn ResetMP
  (MP|SetCurrentMP (Utilities|Struct|BreakSTR_UnitData_Stats (.Stats (Utilities|Struct|BreakSTR_UnitData (Variables|Default|GetUnitData)))) true))

(fn SetCurrentAP
  (params (AP :type Integer) (Show%20Number :type Boolean))
  (bind _unitdata (Variables|Default|GetUnitData))
  (bind _stats (Utilities|Struct|BreakSTR_UnitData _unitdata))
  (bind (_ap_current _ap_max) (Utilities|Struct|BreakSTR_UnitData_Stats _stats))
  (LocalVariables|SetDifference (- AP _ap_current))
  (bind _structout (Utilities|Struct|SetmembersinSTR_UnitData_Stats (Utilities|Struct|BreakSTR_UnitData (Variables|Default|GetUnitData)) (Math|Integer|Clamp(Integer) AP 0 _ap_max)))
  (Utilities|Struct|SetmembersinSTR_UnitData (Variables|Default|GetUnitData) _structout)
  (Default|CallOnUnitStatsChanged self)
  (if (and Show%20Number (!= (LocalVariables|GetDifference) 0))
    (Game|SpawnActorfromClass "/Game/2-Blueprints/Core/Units/Widget/BP_AnimatedNumber.BP_AnimatedNumber_C" (Math|Transform|MakeTransform (Transformation|GetActorLocation) "0, 0, 0" "1.000000,1.000000,1.000000") "Undefined" "MultiplyWithRoot" 0 (LocalVariables|GetDifference) "NewEnumerator3" 0)))

(fn ModifyCurrentAP
  (params (Modifier :type Integer) (Show%20Number :type Boolean))
  (AP|SetCurrentAP (+ Modifier (.AP_Current (Utilities|Struct|BreakSTR_UnitData_Stats (Utilities|Struct|BreakSTR_UnitData (Variables|Default|GetUnitData))))) Show%20Number))

(fn ResetAP
  (AP|SetCurrentAP (.AP_Max (Utilities|Struct|BreakSTR_UnitData_Stats (Utilities|Struct|BreakSTR_UnitData (Variables|Default|GetUnitData)))) true))

(fn CanCastSpell
  (params (Spell%20Data :type STR%20Spell%20Data%20Structure))
  (bind _unitdata (Variables|Default|GetUnitData))
  (bind _stats (Utilities|Struct|BreakSTR_UnitData _unitdata))
  (bind _requirements (Utilities|Struct|BreakSTR_SpellData Spell%20Data))
  (bind _ap_current (Utilities|Struct|BreakSTR_UnitData_Stats _stats))
  (bind _cost_ap (Utilities|Struct|BreakSTR_SpellData_Requirements _requirements))
  (if (Utilities|Array|ContainsItem (Utilities|Struct|BreakSTR_UnitData_Stats (.Stats (Utilities|Struct|BreakSTR_UnitData (Variables|Default|GetUnitData)))) (Utilities|Struct|BreakSTR_SpellData Spell%20Data))
    (Development|PrintString (Utilities|String|Append "AP Current: " (Utilities|String|ToString(Integer) _ap_current)))
    (Development|PrintString (Utilities|String|Append "AP Cost: " (Utilities|String|ToString(Integer) _cost_ap)))
    (if (>= _ap_current (Math|Integer|Absolute(Integer) _cost_ap))
      (return true)
      (else
        (return false)))
    (else
      (return false))))

(fn IsAlive
  (return (> (Utilities|Struct|BreakSTR_UnitData_Stats (Utilities|Struct|BreakSTR_UnitData (Variables|Default|GetUnitData))) 0)))