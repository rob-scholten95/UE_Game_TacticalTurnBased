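; Player action that, after the inherited tile-and-unit selection runs, marks the grid tiles reachable from the selected tile.
; It runs the grid's reachables pathfinder using the selected unit's movement points, diagonal rule and valid tile types, or its own settings without a unit.
; A completion callback applies the tile state to the results.
; Unit walk events clear the highlight on start and regenerate it on finish.
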(event EventBeginPlay
  (|CallParentFunction))

(event Collision|EventActorBeginOverlap
  (params (OtherActor :type Actor%20Object%20Reference))
  (|CallParentFunction OtherActor) ; This node is disabled and will not be called.\nDrag off pins to build functionality.
)

(event EventTick
  (params (DeltaSeconds :type Float%20%28single-precision%29))
  (|CallParentFunction DeltaSeconds))

(fn ConstructionScript
  (|CallParentFunction))

(fn GenerateReachables
  (bind _bp_playeractions (Variables|Default|GetBP_PlayerActions))
  (bind _bp_playeractions_2 (Variables|Default|GetBP_PlayerActions))
  (bind _selectedunit (Variables|/Game/2-Blueprints/Core/Player/BP_PlayerActions.BP_PlayerActions_C|GetSelectedUnit _bp_playeractions))
  (bind _selectedunit_2 (Variables|/Game/2-Blueprints/Core/Player/BP_PlayerActions.BP_PlayerActions_C|GetSelectedUnit _bp_playeractions_2))
  (bind _unitdata (Variables|/Game/2-Blueprints/Core/Units/BP_Unit.BP_Unit_C|GetUnitData _selectedunit))
  (bind _stats (Utilities|Struct|BreakSTR_UnitData _unitdata))
  (bind (_validtiletypes _canmovediagonally _availablespelllist _hp_current _hp_max _mp_current) (Utilities|Struct|BreakSTR_UnitData_Stats _stats))
  (Default|ClearStatefromTiles (Variables|/Game/2-Blueprints/Core/Player/BP_PlayerActions.BP_PlayerActions_C|GetBP_Grid (Variables|Default|GetBP_PlayerActions)) "NewEnumerator7")
  (EventDispatchers|BindEventtoOnPathFindingCompleted (Variables|/Game/2-Blueprints/Core/Grid/BP_Grid.BP_Grid_C|GetBP_GridPathFinding_Reachables (Variables|/Game/2-Blueprints/Core/Player/BP_PlayerActions.BP_PlayerActions_C|GetBP_Grid (Variables|Default|GetBP_PlayerActions))) (EventDispatchers|CreateEvent :!event OnPathFindingCompleted))
  (Utilities|IsValid (Variables|/Game/2-Blueprints/Core/Player/BP_PlayerActions.BP_PlayerActions_C|GetSelectedUnit (Variables|Default|GetBP_PlayerActions))
    (:Is%20Valid
      (EventDispatchers|BindEventtoOnUnitStartWalking _selectedunit_2 (EventDispatchers|CreateEvent :!event OnUnitStartWalking))
      (EventDispatchers|BindEventtoOnUnitFinishedWalking _selectedunit_2 (EventDispatchers|CreateEvent :!event OnUnitStoppedWalking))
      (Default|FindPath (Variables|/Game/2-Blueprints/Core/Grid/BP_Grid.BP_Grid_C|GetBP_GridPathFinding_Reachables (Variables|/Game/2-Blueprints/Core/Player/BP_PlayerActions.BP_PlayerActions_C|GetBP_Grid (Variables|Default|GetBP_PlayerActions))) (Variables|/Game/2-Blueprints/Core/Player/BP_PlayerActions.BP_PlayerActions_C|GetSelectedTileIndex (Variables|Default|GetBP_PlayerActions)) (Utilities|Struct|MakeIntPoint -999 -999) _canmovediagonally 0.0 0.0 _validtiletypes true _mp_current))
    (:Is%20Not%20Valid
      (Default|FindPath (Variables|/Game/2-Blueprints/Core/Grid/BP_Grid.BP_Grid_C|GetBP_GridPathFinding_Reachables (Variables|/Game/2-Blueprints/Core/Player/BP_PlayerActions.BP_PlayerActions_C|GetBP_Grid (Variables|Default|GetBP_PlayerActions))) (Variables|/Game/2-Blueprints/Core/Player/BP_PlayerActions.BP_PlayerActions_C|GetSelectedTileIndex (Variables|Default|GetBP_PlayerActions)) (Utilities|Struct|MakeIntPoint -999 -999) (Variables|Default|GetIncludeDiagonals) (Variables|Default|GetDelayBetweenIterations) (Variables|Default|GetMaxMSPerFrame) (select (Variables|Default|GetIncludeFlyingOnly) (Utilities|Array|MakeArray "NewEnumerator1" "NewEnumerator4" "NewEnumerator5" "NewEnumerator6") (Utilities|Array|MakeArray "NewEnumerator1" "NewEnumerator4" "NewEnumerator5")) true (Variables|Default|GetMaxPathLength)))))

(fn ExecuteAction
  (params (Index :type Int%20Point%20Structure))
  (|CallParentFunction Index)
  (CallFunction|GenerateReachables))

(fn OnPathFindingCompleted
  (params (Path :type Array%20of%20Int%20Point%20Structures))
  (for _array_element Path
    (Default|AddStatetoTile (Variables|/Game/2-Blueprints/Core/Player/BP_PlayerActions.BP_PlayerActions_C|GetBP_Grid (Variables|Default|GetBP_PlayerActions)) _array_element "NewEnumerator7")))

(fn OnUnitStoppedWalking
  (params (Unit :type BP%20Unit%20Object%20Reference))
  (CallFunction|GenerateReachables))

(fn OnUnitStartWalking
  (params (Unit :type BP%20Unit%20Object%20Reference))
  (Default|ClearStatefromTiles (Variables|/Game/2-Blueprints/Core/Player/BP_PlayerActions.BP_PlayerActions_C|GetBP_Grid (Variables|Default|GetBP_PlayerActions)) "NewEnumerator7"))