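; Player action that places a unit of a chosen type and team on a grid tile, or removes the unit standing there.
; When adding, it checks the tile type against the unit type's valid tile types, destroys any existing occupant, then spawns a BP_Unit and registers it with the combat system.
; When removing, it takes any occupant out of combat and destroys it.
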(event EventBeginPlay
  (|CallParentFunction) ; This node is disabled and will not be called.\nDrag off pins to build functionality.
)

(event Collision|EventActorBeginOverlap
  (params (OtherActor :type Actor%20Object%20Reference))
  (|CallParentFunction OtherActor) ; This node is disabled and will not be called.\nDrag off pins to build functionality.
)

(event EventTick
  (params (DeltaSeconds :type Float%20%28single-precision%29))
  (|CallParentFunction DeltaSeconds) ; This node is disabled and will not be called.\nDrag off pins to build functionality.
)

(fn ConstructionScript
  (|CallParentFunction))

(fn ExecuteAction
  (params (Index :type Int%20Point%20Structure))
  (bind _bp_playeractions (Variables|Default|GetBP_PlayerActions))
  (bind _bp_grid (Variables|/Game/2-Blueprints/Core/Player/BP_PlayerActions.BP_PlayerActions_C|GetBP_Grid _bp_playeractions))
  (bind _gridtiles (Variables|/Game/2-Blueprints/Core/Grid/BP_Grid.BP_Grid_C|GetGridTiles _bp_grid))
  (bind _value (Utilities|Map|Find _gridtiles Index))
  (bind _unitontile (Utilities|Struct|BreakSTR_TileData _value))
  (if (Variables|Default|GetIsAddingUnit)
    (bind _unit_data (CallFunction|GetDefaultDatafromUnitType (Variables|Default|GetUnit%20Type)))
    (if (Utilities|Array|ContainsItem (.ValidTileTypes (Utilities|Struct|BreakSTR_UnitData_Stats (.Stats (Utilities|Struct|BreakSTR_UnitData _unit_data)))) (.tiletype (.Value (Utilities|Map|Find (Variables|/Game/2-Blueprints/Core/Grid/BP_Grid.BP_Grid_C|GetGridTiles (Variables|/Game/2-Blueprints/Core/Player/BP_PlayerActions.BP_PlayerActions_C|GetBP_Grid (Variables|Default|GetBP_PlayerActions))) Index))))
      (Utilities|FlowControl|Sequence
        (:then_0
          (Utilities|IsValid _unitontile :!label _label
            (:Is%20Valid
              (Default|RemoveUnitfromCombat (Variables|/Game/2-Blueprints/Core/Player/BP_PlayerActions.BP_PlayerActions_C|GetBP_CombatSystem (Variables|Default|GetBP_PlayerActions)) _unitontile true))))
        (:then_1
          (bind _returnvalue (Game|SpawnActorfromClass "/Game/2-Blueprints/Core/Units/BP_Unit.BP_Unit_C" (Math|Transform|MakeTransform "0, 0, 0" "0, 0, 0" "1.000000,1.000000,1.000000") "Undefined" "MultiplyWithRoot" 0 (Variables|Default|GetUnit%20Type) 0))
          (Default|AddUnittoCombat (Variables|/Game/2-Blueprints/Core/Player/BP_PlayerActions.BP_PlayerActions_C|GetBP_CombatSystem (Variables|Default|GetBP_PlayerActions)) _returnvalue Index (Variables|Default|GetTeamIndex)))))
    (else
      (goto _label))))