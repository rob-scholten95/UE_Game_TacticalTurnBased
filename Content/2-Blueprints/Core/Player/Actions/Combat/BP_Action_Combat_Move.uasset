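; Player combat action for moving the selected unit on the grid, highlighting reachable tiles and previewing a path to the hovered tile.
; Two grid pathfinders return results through completion events that mark tile states, using the unit's movement points, diagonal rule and valid tile types.
; Hovering another unit shows that unit's range instead; executing passes the stored path to the combat system.
; Walk start and finish events pause and then refresh the previews.
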(event EventBeginPlay
  (bind _bp_playeractions (Variables|Default|GetBP_PlayerActions))
  (bind _bp_playeractions_2 (Variables|Default|GetBP_PlayerActions))
  (bind _selectedunit (Variables|/Game/2-Blueprints/Core/Player/BP_PlayerActions.BP_PlayerActions_C|GetSelectedUnit _bp_playeractions))
  (bind _bp_grid (Variables|/Game/2-Blueprints/Core/Player/BP_PlayerActions.BP_PlayerActions_C|GetBP_Grid _bp_playeractions_2))
  (|CallParentFunction)
  (EventDispatchers|BindEventtoOnPathFindingCompleted (Variables|/Game/2-Blueprints/Core/Grid/BP_Grid.BP_Grid_C|GetBP_GridPathFinding_Reachables _bp_grid) (EventDispatchers|CreateEvent :!event OnPathFindingCompletedReachables))
  (EventDispatchers|BindEventtoOnPathFindingCompleted (Variables|/Game/2-Blueprints/Core/Grid/BP_Grid.BP_Grid_C|GetBP_GridPathFinding _bp_grid) (EventDispatchers|CreateEvent :!event OnPathFindingCompletedPath))
  (EventDispatchers|BindEventtoOnUnitStartWalking _selectedunit (EventDispatchers|CreateEvent :!event OnUnitStartedWalking))
  (EventDispatchers|BindEventtoOnUnitFinishedWalking _selectedunit (EventDispatchers|CreateEvent :!event OnUnitFinishedWalking))
  (CallFunction|GenerateReachables (Variables|/Game/2-Blueprints/Core/Player/BP_PlayerActions.BP_PlayerActions_C|GetSelectedUnit (Variables|Default|GetBP_PlayerActions))))

(event EventEndPlay
  (params (EndPlayReason :type EEndPlayReason%20Enum :default "Destroyed"))
  (bind _bp_playeractions (Variables|Default|GetBP_PlayerActions))
  (bind _bp_grid (Variables|/Game/2-Blueprints/Core/Player/BP_PlayerActions.BP_PlayerActions_C|GetBP_Grid _bp_playeractions))
  (|CallParentFunction EndPlayReason)
  (Default|ClearStatefromTiles _bp_grid "NewEnumerator7")
  (Default|ClearStatefromTiles _bp_grid "NewEnumerator4"))

(fn ConstructionScript
  (|CallParentFunction))

(fn GenerateReachables
  (params (Unit :type BP%20Unit%20Object%20Reference))
  (if (!= Unit (Variables|Default|GetCurrentUnitReachables))
    (Variables|Default|SetCurrentUnitReachables Unit)
    (Default|ClearStatefromTiles (Variables|/Game/2-Blueprints/Core/Player/BP_PlayerActions.BP_PlayerActions_C|GetBP_Grid (Variables|Default|GetBP_PlayerActions)) "NewEnumerator7")
    (Default|FindPath (Variables|/Game/2-Blueprints/Core/Grid/BP_Grid.BP_Grid_C|GetBP_GridPathFinding_Reachables (Variables|/Game/2-Blueprints/Core/Player/BP_PlayerActions.BP_PlayerActions_C|GetBP_Grid (Variables|Default|GetBP_PlayerActions))) (Variables|/Game/2-Blueprints/Core/Units/BP_Unit.BP_Unit_C|GetIndex (Variables|Default|GetCurrentUnitReachables)) (Utilities|Struct|MakeIntPoint -999 -999) (.CanMoveDiagonally (Utilities|Struct|BreakSTR_UnitData_Stats (Utilities|Struct|BreakSTR_UnitData (Variables|/Game/2-Blueprints/Core/Units/BP_Unit.BP_Unit_C|GetUnitData (Variables|Default|GetCurrentUnitReachables))))) 0.0 0.0 (.ValidTileTypes (Utilities|Struct|BreakSTR_UnitData_Stats (Utilities|Struct|BreakSTR_UnitData (Variables|/Game/2-Blueprints/Core/Units/BP_Unit.BP_Unit_C|GetUnitData (Variables|Default|GetCurrentUnitReachables))))) true (.MP_Current (Utilities|Struct|BreakSTR_UnitData_Stats (Utilities|Struct|BreakSTR_UnitData (Variables|/Game/2-Blueprints/Core/Units/BP_Unit.BP_Unit_C|GetUnitData (Variables|Default|GetCurrentUnitReachables))))))))

(fn OnPathFindingCompletedReachables
  (params (Reachables :type Array%20of%20Int%20Point%20Structures))
  (if (not (Variables|Default|GetIsUnitWalking))
    (for _array_element Reachables
      (Default|AddStatetoTile (Variables|/Game/2-Blueprints/Core/Player/BP_PlayerActions.BP_PlayerActions_C|GetBP_Grid (Variables|Default|GetBP_PlayerActions)) _array_element "NewEnumerator7"))))

(fn ExecuteHoveredAction
  (params (Index :type Int%20Point%20Structure))
  (bind _bp_playeractions (Variables|Default|GetBP_PlayerActions))
  (bind _hoveredunit (Variables|/Game/2-Blueprints/Core/Player/BP_PlayerActions.BP_PlayerActions_C|GetHoveredUnit _bp_playeractions))
  (|CallParentFunction Index)
  (if (not (Variables|Default|GetIsUnitWalking))
    (Utilities|IsValid _hoveredunit
      (:Is%20Valid
        (CallFunction|GenerateReachables _hoveredunit))
      (:Is%20Not%20Valid
        (CallFunction|GenerateReachables (Variables|/Game/2-Blueprints/Core/Player/BP_PlayerActions.BP_PlayerActions_C|GetSelectedUnit _bp_playeractions))
        (CallFunction|GeneratePath)))))

(fn GeneratePath
  (bind _bp_playeractions (Variables|Default|GetBP_PlayerActions))
  (bind _selectedunit (Variables|/Game/2-Blueprints/Core/Player/BP_PlayerActions.BP_PlayerActions_C|GetSelectedUnit _bp_playeractions))
  (bind _unitdata (Variables|/Game/2-Blueprints/Core/Units/BP_Unit.BP_Unit_C|GetUnitData _selectedunit))
  (bind _stats (Utilities|Struct|BreakSTR_UnitData _unitdata))
  (bind (_validtiletypes _canmovediagonally _mp_current) (Utilities|Struct|BreakSTR_UnitData_Stats _stats))
  (Default|ClearStatefromTiles (Variables|/Game/2-Blueprints/Core/Player/BP_PlayerActions.BP_PlayerActions_C|GetBP_Grid (Variables|Default|GetBP_PlayerActions)) "NewEnumerator4")
  (Utilities|Array|Clear (Variables|Default|GetGeneratedPath))
  (Default|FindPath (Variables|/Game/2-Blueprints/Core/Grid/BP_Grid.BP_Grid_C|GetBP_GridPathFinding (Variables|/Game/2-Blueprints/Core/Player/BP_PlayerActions.BP_PlayerActions_C|GetBP_Grid (Variables|Default|GetBP_PlayerActions))) (Variables|/Game/2-Blueprints/Core/Units/BP_Unit.BP_Unit_C|GetIndex _selectedunit) (Variables|/Game/2-Blueprints/Core/Player/BP_PlayerActions.BP_PlayerActions_C|GetHoveredTileIndex (Variables|Default|GetBP_PlayerActions)) _canmovediagonally 0.0 0.0 _validtiletypes false _mp_current))

(fn OnPathFindingCompletedPath
  (params (Index :type Array%20of%20Int%20Point%20Structures))
  (Variables|Default|SetGeneratedPath Index)
  (for _array_element Index
    (Default|AddStatetoTile (Variables|/Game/2-Blueprints/Core/Player/BP_PlayerActions.BP_PlayerActions_C|GetBP_Grid (Variables|Default|GetBP_PlayerActions)) _array_element "NewEnumerator4")))

(fn ExecuteAction
  (params (Index :type Int%20Point%20Structure))
  (bind _bp_playeractions (Variables|Default|GetBP_PlayerActions))
  (|CallParentFunction Index)
  (if (> (Utilities|Array|Length (Variables|Default|GetGeneratedPath)) 0)
    (Default|MoveUnit (Variables|/Game/2-Blueprints/Core/Player/BP_PlayerActions.BP_PlayerActions_C|GetBP_CombatSystem _bp_playeractions) (Variables|/Game/2-Blueprints/Core/Player/BP_PlayerActions.BP_PlayerActions_C|GetSelectedUnit _bp_playeractions) (Variables|Default|GetGeneratedPath))
    (Utilities|Array|Clear (Variables|Default|GetGeneratedPath))))

(fn OnUnitStartedWalking
  (params (Unit :type BP%20Unit%20Object%20Reference))
  (Variables|Default|SetIsUnitWalking true)
  (Default|ClearStatefromTiles (Variables|/Game/2-Blueprints/Core/Player/BP_PlayerActions.BP_PlayerActions_C|GetBP_Grid (Variables|Default|GetBP_PlayerActions)) "NewEnumerator7")
  (Variables|Default|SetCurrentUnitReachables 0))

(fn OnUnitFinishedWalking
  (params (Unit :type BP%20Unit%20Object%20Reference))
  (Variables|Default|SetIsUnitWalking false)
  (CallFunction|ExecuteHoveredAction (Variables|/Game/2-Blueprints/Core/Player/BP_PlayerActions.BP_PlayerActions_C|GetHoveredTileIndex (Variables|Default|GetBP_PlayerActions))))