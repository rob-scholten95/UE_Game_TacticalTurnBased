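; BP_PlayerActions is the player's input hub for grid-based, turn-based combat, tracking hovered and selected tiles and units.
; Each tick it traces under the cursor, updating tile states and unit highlights.
; Left and right clicks delegate to swappable action actors, spawned per mode and re-executed while dragging across tiles.
; Combat system events drive selection, switch between move and cast-spell actions (number keys pick spells), and manage combat and end-screen widgets.
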(event Custom|OnHoveredTileChange
  (bind _selectedaction_leftclick (Variables|Actions|GetSelectedAction_LeftClick))
  (bind _selectedaction_rightclick (Variables|Actions|GetSelectedAction_RightClick))
  (Utilities|FlowControl|Sequence
    (:then_0
      (Utilities|IsValid _selectedaction_leftclick
        (:Is%20Valid
          (Default|ExecuteHoveredAction _selectedaction_leftclick)
          (if (Variables|Controls|GetIsLeftClickDown)
            (Default|ExecuteAction (Variables|Actions|GetSelectedAction_LeftClick) (Variables|TileSelection|GetHoveredTileIndex))))))
    (:then_1
      (Utilities|IsValid _selectedaction_rightclick
        (:Is%20Valid
          (Default|ExecuteHoveredAction _selectedaction_rightclick)
          (if (Variables|Controls|GetIsRightClickDown)
            (Default|ExecuteAction (Variables|Actions|GetSelectedAction_RightClick) (Variables|TileSelection|GetHoveredTileIndex))))))))

(event Input|EnhancedActionEvents|EnhancedInputActionIA_Click_Left
  (params (ActionValue :type Boolean) (ElapsedSeconds :type Float%20%28double-precision%29) (TriggeredSeconds :type Float%20%28double-precision%29) (InputAction :type Input%20Action%20Object%20Reference :default "/Game/3-Input/InputActions/IA_Click_Left.IA_Click_Left"))
  (:Triggered
    (CallFunction|UpdateTileandUnitUnderCursor)
    (Variables|Controls|SetIsLeftClickDown true)
    (Utilities|IsValid (Variables|Actions|GetSelectedAction_LeftClick)
      (:Is%20Valid
        (Default|ExecuteAction (Variables|Actions|GetSelectedAction_LeftClick) (Variables|TileSelection|GetHoveredTileIndex)))))
  (:Canceled
    (Variables|Controls|SetIsLeftClickDown false :!label _label))
  (:Completed
    (goto _label)))

(event Input|EnhancedActionEvents|EnhancedInputActionIA_Click_Right
  (params (ActionValue :type Boolean) (ElapsedSeconds :type Float%20%28double-precision%29) (TriggeredSeconds :type Float%20%28double-precision%29) (InputAction :type Input%20Action%20Object%20Reference :default "/Game/3-Input/InputActions/IA_Click_Right.IA_Click_Right"))
  (:Triggered
    (CallFunction|UpdateTileandUnitUnderCursor)
    (Variables|Controls|SetIsRightClickDown true)
    (Utilities|IsValid (Variables|Actions|GetSelectedAction_RightClick)
      (:Is%20Valid
        (Default|ExecuteAction (Variables|Actions|GetSelectedAction_RightClick) (Variables|TileSelection|GetHoveredTileIndex)))))
  (:Canceled
    (Variables|Controls|SetIsRightClickDown false :!label _label))
  (:Completed
    (goto _label)))

(event EventBeginPlay
  (Utilities|FlowControl|Sequence
    (:then_0
      ;[1 1 1] Comment
      (bind _returnvalue (Actor|GetActorOfClass "/Game/2-Blueprints/Core/Grid/BP_Grid.BP_Grid_C"))
      (Utilities|IsValid _returnvalue
        (:Is%20Valid
          (Variables|Refs|SetBP_Grid _returnvalue)
          (EventDispatchers|BindEventtoOnGridGenerated (Variables|Refs|GetBP_Grid) (EventDispatchers|CreateEvent :!event OnGridGenerated))
          (EventDispatchers|BindEventtoOnTileDataUpdated (Variables|Refs|GetBP_Grid) (EventDispatchers|CreateEvent :!event OnTileDataUpdated)))))
    (:then_1
      ;;[1 1 1] Comment
      (Variables|Refs|SetPC_Game (Game|GetPlayerController 0)))
    (:then_2
      ;[1 1 1] Comment
      (Utilities|IsValid (PlayerController|LocalPlayerSubsystems|GetEnhancedInputLocalPlayerSubsystem (Variables|Refs|GetPC_Game))
        (:Is%20Valid
          (Input|AddMappingContext (PlayerController|LocalPlayerSubsystems|GetEnhancedInputLocalPlayerSubsystem (Variables|Refs|GetPC_Game)) "/Game/3-Input/IMC_PLayerControls.IMC_PLayerControls" 0 (Utilities|Struct|MakeModifyContextOptions true false)))))
    (:then_3
      ;[1 1 1] Comment
      (bind _returnvalue_2 (Actor|GetActorOfClass "BP_PlayerActions_C"))
      (Utilities|IsValid _returnvalue_2
        (:Is%20Valid
          (Variables|Refs|SetBP_PlayerActions _returnvalue_2))))
    (:then_4
      ;[1 1 1] Comment
      (bind _returnvalue_3 (Actor|GetActorOfClass "/Game/2-Blueprints/Core/Combat/BP_CombatSystem.BP_CombatSystem_C"))
      (Utilities|IsValid _returnvalue_3
        (:Is%20Valid
          (bind _output_get (Variables|Refs|SetBP_CombatSystem _returnvalue_3))
          (EventDispatchers|BindEventtoOnUnitGridIndexChanged _output_get (EventDispatchers|CreateEvent :!event OnUnitGridIndexChanged))
          (EventDispatchers|BindEventtoOnCombatStarted (Variables|Refs|GetBP_CombatSystem) (EventDispatchers|CreateEvent :!event OnCombatStarted))
          (EventDispatchers|BindEventtoOnCombatEnded (Variables|Refs|GetBP_CombatSystem) (EventDispatchers|CreateEvent :!event OnCombatEnded))
          (EventDispatchers|AssignOnUnitTurnStarted (Variables|Refs|GetBP_CombatSystem) (EventDispatchers|CreateEvent :!event OnUnitTurnStarted))
          (EventDispatchers|AssignOnUnitTurnEnded (Variables|Refs|GetBP_CombatSystem) (EventDispatchers|CreateEvent :!event OnUnitTurnEnded))
          (EventDispatchers|BindEventtoOnCombatFinishing (Variables|Refs|GetBP_CombatSystem) (EventDispatchers|CreateEvent :!event OnCombatFinishing))
          (Input|EnableInput (Game|GetPlayerController 0)))))))

(event EventTick
  (params (DeltaSeconds :type Float%20%28single-precision%29))
  (CallFunction|UpdateTileandUnitUnderCursor))

(event Input|KeyboardEvents|AnyKey
  (params (Key :type Key%20Structure :default "None"))
  (bind _returnvalue (Class|KismetInputLibrary|KeyGetDisplayName Key true))
  (bind _bp_combatsystem (Variables|Refs|GetBP_CombatSystem))
  (bind _returnvalue_2 (Utilities|String|ToString(Text) _returnvalue))
  ;[1 1 1] Comment
  (:Pressed
    (if (and (Variables|/Game/2-Blueprints/Core/Combat/BP_CombatSystem.BP_CombatSystem_C|GetIsInCombat _bp_combatsystem) (not (Variables|/Game/2-Blueprints/Core/Combat/BP_CombatSystem.BP_CombatSystem_C|GetIsFinishingCombat _bp_combatsystem)))
      (if (Class|KismetStringLibrary|IsNumeric _returnvalue_2)
        (Default|SetSelectedSpellfromIndex (Variables|/Game/2-Blueprints/Core/Combat/Widgets/UW_Combat.UW_Combat_C|GetUW_Button_ListSpells (Variables|Refs|GetUW_Combat)) (- (Math|Conversions|ToInteger(Byte) _returnvalue_2) 1))))))

(fn ConstructionScript)

(fn UpdateTileandUnitUnderCursor
  (Utilities|FlowControl|Sequence
    (:then_0
      (bind _asbp_unit (CallFunction|GetUnitUnderCursor))
      (if (!= _asbp_unit (Variables|UnitSelection|GetHoveredUnit))
        (Utilities|FlowControl|Sequence
          (:then_0
            (Utilities|IsValid (Variables|UnitSelection|GetHoveredUnit)
              (:Is%20Valid
                (Default|SetIsHovered (Variables|UnitSelection|GetHoveredUnit) false))))
          (:then_1
            (bind _output_get (Variables|UnitSelection|SetHoveredUnit _asbp_unit))
            (Utilities|IsValid _output_get
              (:Is%20Valid
                (Default|SetIsHovered _output_get true)))))))
    (:then_1
      (Utilities|IsValid (Variables|UnitSelection|GetHoveredUnit)
        (:Is%20Valid
          (LocalVariables|SetNew%20Index (Variables|/Game/2-Blueprints/Core/Units/BP_Unit.BP_Unit_C|GetIndex (Variables|UnitSelection|GetHoveredUnit))))
        (:Is%20Not%20Valid
          (bind _index (Default|GetTileIndexUnderCursor (Variables|Refs|GetBP_Grid)))
          (LocalVariables|SetNew%20Index _index)))
      (if (!= (LocalVariables|GetNew%20Index) (Variables|TileSelection|GetHoveredTileIndex))
        (Default|RemoveStatefromTile (Variables|Refs|GetBP_Grid) (Variables|TileSelection|GetHoveredTileIndex) "NewEnumerator1")
        (Variables|TileSelection|SetHoveredTileIndex (LocalVariables|GetNew%20Index))
        (Default|AddStatetoTile (Variables|Refs|GetBP_Grid) (Variables|TileSelection|GetHoveredTileIndex) "NewEnumerator1")
        (CallFunction|OnHoveredTileChange)))))

(fn SetSelectedActions
  (params (LeftAction :type BP%20Action%20Class%20Reference) (RightAction :type BP%20Action%20Class%20Reference))
  (Utilities|FlowControl|Sequence
    (:then_0
      (Utilities|IsValid (Variables|Actions|GetSelectedAction_LeftClick)
        (:Is%20Valid
          (Actor|DestroyActor (Variables|Actions|GetSelectedAction_LeftClick))
          (Variables|Actions|SetSelectedAction_LeftClick 0))
        (:Is%20Not%20Valid
          _))
      (if (Utilities|IsValidClass LeftAction)
        (bind _returnvalue (Game|SpawnActorfromClass LeftAction (Math|Transform|MakeTransform "0, 0, 0" "0, 0, 0" "1.000000,1.000000,1.000000") "AlwaysSpawn" "MultiplyWithRoot" 0 self 0))
        (Variables|Actions|SetSelectedAction_LeftClick _returnvalue)))
    (:then_1
      (Utilities|IsValid (Variables|Actions|GetSelectedAction_RightClick)
        (:Is%20Valid
          (Actor|DestroyActor (Variables|Actions|GetSelectedAction_RightClick))
          (Variables|Actions|SetSelectedAction_RightClick 0))
        (:Is%20Not%20Valid
          _))
      (if (Utilities|IsValidClass RightAction)
        (bind _returnvalue_2 (Game|SpawnActorfromClass RightAction (Math|Transform|MakeTransform "0, 0, 0" "0, 0, 0" "1.000000,1.000000,1.000000") "AlwaysSpawn" "MultiplyWithRoot" 0 self 0))
        (Variables|Actions|SetSelectedAction_RightClick _returnvalue_2)))
    (:then_2
      (Default|CallOnSelectedActionsChanged (Variables|Actions|GetSelectedAction_LeftClick) (Variables|Actions|GetSelectedAction_RightClick)))))

(fn GetUnitUnderCursor
  (params (Player%20Index :type Integer))
  (bind _returnvalue (Game|GetPlayerController 0))
  (bind (_hitresult _returnvalue_2) (Game|Player|GetHitResultUnderCursorbyChannel _returnvalue "TraceTypeQuery5" true))
  (if _returnvalue_2
    (return (.AsBP%20Unit (Utilities|Casting|CastToBP_Unit (.HitActor (Collision|BreakHitResult _hitresult)))))
    (else
      (bind _index (Default|GetTileIndexUnderCursor (Variables|Refs|GetBP_Grid) Player%20Index))
      (return (Utilities|Struct|BreakSTR_TileData (.Value (Utilities|Map|Find (Variables|/Game/2-Blueprints/Core/Grid/BP_Grid.BP_Grid_C|GetGridTiles (Variables|Refs|GetBP_Grid)) _index)))))))

(fn SetSelectedTileandUnit
  (params (Index :type Int%20Point%20Structure) (Force :type Boolean))
  (Utilities|FlowControl|Sequence
    (:then_0
      (if (or Force (!= (Variables|TileSelection|GetSelectedTileIndex) Index))
        (Default|RemoveStatefromTile (Variables|Refs|GetBP_Grid) (Variables|TileSelection|GetSelectedTileIndex) "NewEnumerator2")
        (Variables|TileSelection|SetSelectedTileIndex Index)
        (Default|AddStatetoTile (Variables|Refs|GetBP_Grid) (Variables|TileSelection|GetSelectedTileIndex) "NewEnumerator2")
        (else
          (Default|RemoveStatefromTile (Variables|Refs|GetBP_Grid) (Variables|TileSelection|GetSelectedTileIndex) "NewEnumerator2")
          (Variables|TileSelection|SetSelectedTileIndex (Utilities|Struct|MakeIntPoint -999 -999))))
      (Default|CallOnSelecteTileChanged (Variables|TileSelection|GetSelectedTileIndex)))
    (:then_1
      (LocalVariables|SetNew%20Unit (.UnitOnTile (Utilities|Struct|BreakSTR_TileData (.Value (Utilities|Map|Find (Variables|/Game/2-Blueprints/Core/Grid/BP_Grid.BP_Grid_C|GetGridTiles (Variables|Refs|GetBP_Grid)) Index)))))
      (if (or Force (!= (Variables|UnitSelection|GetSelectedUnit) (LocalVariables|GetNew%20Unit)))
        (Utilities|FlowControl|Sequence
          (:then_0
            (Utilities|IsValid (Variables|UnitSelection|GetSelectedUnit)
              (:Is%20Valid
                (Default|SetIsSelected (Variables|UnitSelection|GetSelectedUnit) false))))
          (:then_1
            (bind _output_get (Variables|UnitSelection|SetSelectedUnit (LocalVariables|GetNew%20Unit)))
            (Utilities|IsValid _output_get
              (:Is%20Valid
                (Default|SetIsSelected _output_get true)))))))))

(fn OnGridGenerated
  (if (Default|IsIndexValid (Variables|Refs|GetBP_Grid) (Variables|TileSelection|GetSelectedTileIndex))
    (CallFunction|SetSelectedTileandUnit (Variables|TileSelection|GetSelectedTileIndex) true)
    (else
      (CallFunction|SetSelectedTileandUnit (Utilities|Struct|MakeIntPoint -999 -999) true))))

(fn OnTileDataUpdated
  (params (Index :type Int%20Point%20Structure))
  (if (Class|KismetMathLibrary|EqualIntPointIntPoint Index (Variables|TileSelection|GetSelectedTileIndex))
    (CallFunction|OnGridGenerated)))

(fn OnUnitTurnStarted
  (params (Unit :type BP%20Unit%20Object%20Reference))
  (CallFunction|SetSelectedTileandUnit (Variables|/Game/2-Blueprints/Core/Units/BP_Unit.BP_Unit_C|GetIndex Unit) false)
  (CallFunction|SetSelectedActions "/Game/2-Blueprints/Core/Player/Actions/Combat/BP_Action_Combat_Move.BP_Action_Combat_Move_C")
  (Default|LinkUnittoSpellsList (Variables|/Game/2-Blueprints/Core/Combat/Widgets/UW_Combat.UW_Combat_C|GetUW_Button_ListSpells (Variables|Refs|GetUW_Combat)) (Variables|UnitSelection|GetSelectedUnit)))

(fn OnUnitGridIndexChanged
  (params (Unit :type BP%20Unit%20Object%20Reference))
  (if (== Unit (Variables|UnitSelection|GetSelectedUnit))
    (CallFunction|SetSelectedTileandUnit (Variables|/Game/2-Blueprints/Core/Units/BP_Unit.BP_Unit_C|GetIndex Unit) false)))

(fn OnCombatStarted
  (CallFunction|SetSelectedActions)
  (CallFunction|SetSelectedTileandUnit (Utilities|Struct|MakeIntPoint -999 -999) false)
  (bind _returnvalue (UserInterface|CreateWidget "/Game/2-Blueprints/Core/Combat/Widgets/UW_Combat.UW_Combat_C" 0 self))
  (bind _output_get (Variables|Refs|SetUW_Combat _returnvalue))
  (UserInterface|Viewport|AddtoPlayerScreen _output_get)
  (EventDispatchers|BindEventtoOnSelectedSpellButtonChanged (Variables|/Game/2-Blueprints/Core/Combat/Widgets/UW_Combat.UW_Combat_C|GetUW_Button_ListSpells (Variables|Refs|GetUW_Combat)) (EventDispatchers|CreateEvent :!event OnSelectedSpellChanged)))

(fn OnCombatEnded
  (bind _uw_combatendscreen (Variables|Refs|GetUW_CombatEndScreen))
  (Widget|RemovefromParent _uw_combatendscreen)
  (Widget|SetVisibility _uw_combatendscreen "Hidden"))

(fn OnUnitTurnEnded
  (params (Unit :type BP%20Unit%20Object%20Reference))
  (CallFunction|SetSelectedTileandUnit (Utilities|Struct|MakeIntPoint -999 -999) false)
  (CallFunction|SetSelectedActions "/Game/2-Blueprints/Core/Player/Actions/Combat/BP_Action_Combat_Move.BP_Action_Combat_Move_C"))

(fn OnSelectedSpellChanged
  (params (SelectedButton :type UW%20Button%20Spell%20Object%20Reference))
  (Utilities|IsValid SelectedButton
    (:Is%20Valid
      (CallFunction|SetSelectedActions "/Game/2-Blueprints/Core/Player/Actions/Combat/BP_Action_Combat_CastSpell.BP_Action_Combat_CastSpell_C")
      (bind _asbp_action_combat_cast_spell (Utilities|Casting|CastToBP_Action_Combat_CastSpell (Variables|Actions|GetSelectedAction_LeftClick)))
      (Default|SetSpell _asbp_action_combat_cast_spell (Variables|/Game/2-Blueprints/Core/Combat/Spells/Widgets/UW_Button_Spell.UW_Button_Spell_C|GetSpell SelectedButton)))
    (:Is%20Not%20Valid
      (if (!= (Utilities|GetClass (Variables|Actions|GetSelectedAction_LeftClick)) "/Game/2-Blueprints/Core/Player/Actions/Combat/BP_Action_Combat_Move.BP_Action_Combat_Move_C")
        (CallFunction|SetSelectedActions "/Game/2-Blueprints/Core/Player/Actions/Combat/BP_Action_Combat_Move.BP_Action_Combat_Move_C")))))

(fn OnCombatFinishing
  (params (Winning%20Team%20Index :type Integer))
  (CallFunction|SetSelectedActions)
  (CallFunction|SetSelectedTileandUnit (Utilities|Struct|MakeIntPoint -999 -999) false)
  (Widget|RemovefromParent (Variables|Refs|GetUW_Combat))
  (Variables|Refs|SetUW_Combat 0)
  (bind _returnvalue (UserInterface|CreateWidget "/Game/2-Blueprints/Core/Combat/Widgets/UW_Combat_EndScreen.UW_Combat_EndScreen_C" 0 self Winning%20Team%20Index))
  (bind _output_get (Variables|Refs|SetUW_CombatEndScreen _returnvalue))
  (UserInterface|Viewport|AddtoPlayerScreen _output_get))