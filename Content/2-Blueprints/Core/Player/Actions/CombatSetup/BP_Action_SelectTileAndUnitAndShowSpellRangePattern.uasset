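; A player action that, on tile selection, previews a spell's range and area-of-effect patterns on the combat grid.
; On execute, it asks the combat system for the range from the selected tile and marks those tiles with a grid state.
; On hover, it marks the AOE range around the hovered tile, or just that tile, only while it lies within the range.
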(event EventBeginPlay
  (|CallParentFunction) ; This node is disabled and will not be called.\nDrag off pins to build functionality.
)

(event Collision|EventActorBeginOverlap
  (params (OtherActor :type Actor%20Object%20Reference))
  (|CallParentFunction OtherActor) ; This node is disabled and will not be called.\nDrag off pins to build functionality.
)

(event EventTick
  (params (DeltaSeconds :type Float%20%28single-precision%29))
  (|CallParentFunction DeltaSeconds) ; This node is disabled and will not be called.\nDrag off pins to build functionality.
)

(fn ConstructionScript
  (|CallParentFunction))

(fn ShowSpellRangePattern
  (bind _bp_playeractions (Variables|Default|GetBP_PlayerActions))
  (bind _bp_playeractions_2 (Variables|Default|GetBP_PlayerActions))
  (Utilities|FlowControl|Sequence
    (:then_0
      (Default|ClearStatefromTiles (Variables|/Game/2-Blueprints/Core/Player/BP_PlayerActions.BP_PlayerActions_C|GetBP_Grid (Variables|Default|GetBP_PlayerActions)) "NewEnumerator8")
      (if (Default|IsIndexValid (Variables|/Game/2-Blueprints/Core/Player/BP_PlayerActions.BP_PlayerActions_C|GetBP_Grid _bp_playeractions) (Variables|/Game/2-Blueprints/Core/Player/BP_PlayerActions.BP_PlayerActions_C|GetSelectedTileIndex _bp_playeractions))
        (bind _range_indexes (Default|GetSpellRange (Variables|/Game/2-Blueprints/Core/Player/BP_PlayerActions.BP_PlayerActions_C|GetBP_CombatSystem _bp_playeractions_2) (Variables|/Game/2-Blueprints/Core/Player/BP_PlayerActions.BP_PlayerActions_C|GetSelectedTileIndex _bp_playeractions_2) (Variables|Default|GetCast)))
        (for _array_element _range_indexes
          (Default|AddStatetoTile (Variables|/Game/2-Blueprints/Core/Player/BP_PlayerActions.BP_PlayerActions_C|GetBP_Grid (Variables|Default|GetBP_PlayerActions)) _array_element "NewEnumerator8"))))
    (:then_1
      (CallFunction|ShowSpellRangePatternAOE))))

(fn ExecuteAction
  (params (Index :type Int%20Point%20Structure))
  (|CallParentFunction Index)
  (CallFunction|ShowSpellRangePattern))

(fn ShowSpellRangePatternAOE
  (bind _bp_playeractions (Variables|Default|GetBP_PlayerActions))
  (Default|ClearStatefromTiles (Variables|/Game/2-Blueprints/Core/Player/BP_PlayerActions.BP_PlayerActions_C|GetBP_Grid (Variables|Default|GetBP_PlayerActions)) "NewEnumerator9")
  (if (Utilities|Array|ContainsItem (Utilities|Struct|BreakSTR_IntPointArray (.Value (Utilities|Map|Find (Variables|/Game/2-Blueprints/Core/Grid/BP_Grid.BP_Grid_C|GetTileStateToIndexes (Variables|/Game/2-Blueprints/Core/Player/BP_PlayerActions.BP_PlayerActions_C|GetBP_Grid (Variables|Default|GetBP_PlayerActions))) "NewEnumerator8"))) (Variables|/Game/2-Blueprints/Core/Player/BP_PlayerActions.BP_PlayerActions_C|GetHoveredTileIndex (Variables|Default|GetBP_PlayerActions)))
    (if (Utilities|Enum|NotEqual(Enum) (.RangePattern (Utilities|Struct|BreakSTR_SpellData_Cast (Variables|Default|GetCast_AOE))) "NewEnumerator0")
      (bind _range_indexes (Default|GetSpellRange (Variables|/Game/2-Blueprints/Core/Player/BP_PlayerActions.BP_PlayerActions_C|GetBP_CombatSystem _bp_playeractions) (Variables|/Game/2-Blueprints/Core/Player/BP_PlayerActions.BP_PlayerActions_C|GetHoveredTileIndex _bp_playeractions) (Variables|Default|GetCast_AOE)))
      (for _array_element _range_indexes
        (Default|AddStatetoTile (Variables|/Game/2-Blueprints/Core/Player/BP_PlayerActions.BP_PlayerActions_C|GetBP_Grid (Variables|Default|GetBP_PlayerActions)) _array_element "NewEnumerator9"))
      (else
        (Default|AddStatetoTile (Variables|/Game/2-Blueprints/Core/Player/BP_PlayerActions.BP_PlayerActions_C|GetBP_Grid (Variables|Default|GetBP_PlayerActions)) (Variables|/Game/2-Blueprints/Core/Player/BP_PlayerActions.BP_PlayerActions_C|GetHoveredTileIndex (Variables|Default|GetBP_PlayerActions)) "NewEnumerator9")))))

(fn ExecuteHoveredAction
  (params (Index :type Int%20Point%20Structure))
  (|CallParentFunction Index)
  (CallFunction|ShowSpellRangePatternAOE))