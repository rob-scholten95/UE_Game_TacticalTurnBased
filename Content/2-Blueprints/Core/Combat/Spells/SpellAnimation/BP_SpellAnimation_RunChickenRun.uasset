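; Spell animation actor that shows the Run Chicken Run icon effect on a target tile.
; When played, it moves to the target tile and sets the icon texture on its widget component's image.
; A timeline animates the widget's height, draw size and opacity.
; A one-time gate signals the tile hit early in playback, and the timeline's end completes the spell animation.
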(event EventBeginPlay
  (|CallParentFunction) ; This node is disabled and will not be called.\nDrag off pins to build functionality.
)

(event Collision|EventActorBeginOverlap
  (params (OtherActor :type Actor%20Object%20Reference)))

(event EventTick
  (params (DeltaSeconds :type Float%20%28single-precision%29)))

(event EventEventPlaySpellAnimation
  (Transformation|SetActorLocation (.location (CallFunction|GetTileTransform (Variables|Default|GetTargetIndex))) false false)
  (bind _output_get (Variables|Default|SetAs%20UW%20Image (.AsUW%20Image (Utilities|Casting|CastToUW_Image (UserInterface|GetUserWidgetObject (Variables|Default|GetWidget))))))
  (Appearance|SetBrushfromTexture (Variables|/Game/2-Blueprints/Core/Combat/Spells/SpellAnimation/Components/UW_Image.UW_Image_C|GetImage_Component _output_get) "/Game/2-Blueprints/Core/Combat/Spells/SpellAnimation/Assets/Icon_RunChickenRun_NoBackground.Icon_RunChickenRun_NoBackground" false)
  (bind (_direction _locationz _draw_size _opacity) (Timeline|Timeline PlayFromStart)
    (:Update
      (Transformation|SetRelativeLocation (Variables|Default|GetWidget) (Math|Vector|MakeVector 0.0 0.0 _locationz) false false)
      (Class|WidgetComponent|SetDrawSize (Variables|Default|GetWidget) (Math|Vector2D|MakeVector2D _draw_size _draw_size))
      (Widget|SetRenderOpacity (Variables|Default|GetAs%20UW%20Image) _opacity)
      (if (>= (Components|Timeline|GetPlaybackPosition (Variables|Default|GetTimeline)) 0.2)
        (Utilities|FlowControl|DoOnce false
          (:Completed
            (Default|CallOnSpellAnimationHitTile self (Variables|Default|GetTargetIndex))))))
    (:Finished
      (CallFunction|EventCompleteSpellAnimation))))

(fn ConstructionScript
  (|CallParentFunction))