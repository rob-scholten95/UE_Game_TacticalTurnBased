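; Player action that finds a grid path from the selected tile to a target tile and marks its tiles.
; Execution clears the previous path state, then runs the grid pathfinding component with configurable diagonals, length, time budget, iteration delay and optional flying-only tile type.
; A completion callback adds the state to each path tile.
; Selection changes and EndPlay re-execute it with a -999 sentinel target.
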(event Custom|OnSelectedTileChanged
  (params (Index :type Int%20Point%20Structure))
  (CallFunction|ExecuteAction (Utilities|Struct|MakeIntPoint -999 -999)))

(event EventBeginPlay
  (EventDispatchers|AssignOnSelecteTileChanged (Variables|Default|GetBP_PlayerActions) (delegate Custom|OnSelectedTileChanged)))

(event EventEndPlay
  (params (EndPlayReason :type EEndPlayReason%20Enum :default "Destroyed"))
  (CallFunction|ExecuteAction (Utilities|Struct|MakeIntPoint -999 -999)))

(fn ConstructionScript
  (|CallParentFunction))

(fn ExecuteAction
  (params (Index :type Int%20Point%20Structure))
  (Default|ClearStatefromTiles (Variables|/Game/2-Blueprints/Core/Player/BP_PlayerActions.BP_PlayerActions_C|GetBP_Grid (Variables|Default|GetBP_PlayerActions)) "NewEnumerator4")
  (EventDispatchers|BindEventtoOnPathFindingCompleted (Variables|/Game/2-Blueprints/Core/Grid/BP_Grid.BP_Grid_C|GetBP_GridPathFinding (Variables|/Game/2-Blueprints/Core/Player/BP_PlayerActions.BP_PlayerActions_C|GetBP_Grid (Variables|Default|GetBP_PlayerActions))) (EventDispatchers|CreateEvent :!event OnPathFindingCompleted))
  (Default|FindPath (Variables|/Game/2-Blueprints/Core/Grid/BP_Grid.BP_Grid_C|GetBP_GridPathFinding (Variables|/Game/2-Blueprints/Core/Player/BP_PlayerActions.BP_PlayerActions_C|GetBP_Grid (Variables|Default|GetBP_PlayerActions))) (Variables|/Game/2-Blueprints/Core/Player/BP_PlayerActions.BP_PlayerActions_C|GetSelectedTileIndex (Variables|Default|GetBP_PlayerActions)) Index (Variables|Default|GetInclude%20Diagonals) (Variables|Default|GetDelay%20Between%20Iterations) (Variables|Default|GetMax%20MSPer%20Frame) (select (Variables|Default|GetIncludeFlyingOnly) (Utilities|Array|MakeArray "NewEnumerator1" "NewEnumerator4" "NewEnumerator5" "NewEnumerator6") (Utilities|Array|MakeArray "NewEnumerator1" "NewEnumerator4" "NewEnumerator5")) false (Variables|Default|GetMaxPathLength)))

(fn OnPathFindingCompleted
  (params (Path :type Array%20of%20Int%20Point%20Structures))
  (for _array_element Path
    (Default|AddStatetoTile (Variables|/Game/2-Blueprints/Core/Player/BP_PlayerActions.BP_PlayerActions_C|GetBP_Grid (Variables|Default|GetBP_PlayerActions)) _array_element "NewEnumerator4")))