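; BP_Action_CastSpell is a player action in combat setup that casts a spell at a chosen tile index.
; Execute Action asks the combat system, reached through the player actions object, to cast its Spell from the selected tile to the given index.
; It then resets the selected unit's MP if that unit is valid.
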(event EventBeginPlay
  (|CallParentFunction) ; This node is disabled and will not be called.\nDrag off pins to build functionality.
)

(event Collision|EventActorBeginOverlap
  (params (OtherActor :type Actor%20Object%20Reference))
  (|CallParentFunction OtherActor) ; This node is disabled and will not be called.\nDrag off pins to build functionality.
)

(event EventTick
  (params (DeltaSeconds :type Float%20%28single-precision%29))
  (|CallParentFunction DeltaSeconds) ; This node is disabled and will not be called.\nDrag off pins to build functionality.
)

(fn ConstructionScript
  (|CallParentFunction))

(fn ExecuteAction
  (params (Index :type Int%20Point%20Structure))
  (bind _bp_playeractions (Variables|Default|GetBP_PlayerActions))
  (bind _selectedunit (Variables|/Game/2-Blueprints/Core/Player/BP_PlayerActions.BP_PlayerActions_C|GetSelectedUnit _bp_playeractions))
  (Default|CastSpell (Variables|/Game/2-Blueprints/Core/Player/BP_PlayerActions.BP_PlayerActions_C|GetBP_CombatSystem (Variables|Default|GetBP_PlayerActions)) (Variables|Default|GetSpell) (Variables|/Game/2-Blueprints/Core/Player/BP_PlayerActions.BP_PlayerActions_C|GetSelectedTileIndex (Variables|Default|GetBP_PlayerActions)) Index)
  (Utilities|IsValid _selectedunit
    (:Is%20Valid
      (Default|ResetMP _selectedunit))))