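; BP_Action_SetTypeTile is a grid player action that sets the tile type of the tile at a given index.
; On execute, it validates the index against the grid owned by the player actions object and looks up that tile's data.
; It then re-adds the tile through AddGridTile with the action's tile type, preserving its index, transform, state and occupying unit.
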(fn ConstructionScript
  (|CallParentFunction))

(fn ExecuteAction
  (params (Index :type Int%20Point%20Structure))
  (if (Default|IsIndexValid (Variables|/Game/2-Blueprints/Core/Player/BP_PlayerActions.BP_PlayerActions_C|GetBP_Grid (Variables|Default|GetBP_PlayerActions)) Index)
    (LocalVariables|SetData (.Value (Utilities|Map|Find (Variables|/Game/2-Blueprints/Core/Grid/BP_Grid.BP_Grid_C|GetGridTiles (Variables|/Game/2-Blueprints/Core/Player/BP_PlayerActions.BP_PlayerActions_C|GetBP_Grid (Variables|Default|GetBP_PlayerActions))) Index)))
    (Default|AddGridTile (Variables|/Game/2-Blueprints/Core/Player/BP_PlayerActions.BP_PlayerActions_C|GetBP_Grid (Variables|Default|GetBP_PlayerActions)) (Utilities|Struct|MakeSTR_TileData (.index (LocalVariables|GetData)) (Variables|Default|GetData%20Tile%20Type) (.transform (LocalVariables|GetData)) (.tilestate (LocalVariables|GetData)) (.unitontile (LocalVariables|GetData))))))