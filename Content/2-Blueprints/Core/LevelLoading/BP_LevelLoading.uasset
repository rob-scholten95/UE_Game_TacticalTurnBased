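; BP_LevelLoading is a Blueprint that switches the active streaming sublevel, keeping track of it in LevelLoaded.
; LoadLevel flags the previous sublevel to unload and hide, stores the requested one, then flags it to load and show.
; It skips requests for the current level unless forced, which BeginPlay does to apply the initial LevelLoaded value.
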(event EventBeginPlay
  (CallFunction|LoadLevel (Variables|Default|GetLevelLoaded) true))

(fn ConstructionScript)

(fn LoadLevel
  (params (Level :type String) (Force :type Boolean))
  (if (or Force (Utilities|Enum|NotEqual(Enum) Level (Variables|Default|GetLevelLoaded)))
    (Utilities|FlowControl|Sequence
      (:then_0
        (Utilities|IsValid (Class|GameplayStatics|GetStreamingLevel (Utilities|String|StringToName (Variables|Default|GetLevelLoaded)))
          (:Is%20Valid
            (Variables|/Script/Engine.LevelStreaming|SetbShouldBeLoaded (Class|GameplayStatics|GetStreamingLevel (Utilities|String|StringToName (Variables|Default|GetLevelLoaded))) false)
            (Variables|/Script/Engine.LevelStreaming|SetbShouldBeVisible (Class|GameplayStatics|GetStreamingLevel (Utilities|String|StringToName (Variables|Default|GetLevelLoaded))) false))))
      (:then_1
        (bind _output_get (Variables|Default|SetLevelLoaded Level))
        (Utilities|IsValid (Class|GameplayStatics|GetStreamingLevel (Utilities|String|StringToName _output_get))
          (:Is%20Valid
            (Variables|/Script/Engine.LevelStreaming|SetbShouldBeLoaded (Class|GameplayStatics|GetStreamingLevel (Utilities|String|StringToName _output_get)) true)
            (Variables|/Script/Engine.LevelStreaming|SetbShouldBeVisible (Class|GameplayStatics|GetStreamingLevel (Utilities|String|StringToName _output_get)) true)))))))